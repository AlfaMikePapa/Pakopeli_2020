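; Client-side pawn for a minigame where a robot moves over a spawned board structure and descends through holes.
; On remote clients, BeginPlay spawns the board, WASD moves the robot, and key 1 rotates the middle stage.
; A touch widget drives height-clamped camera dragging and slider zoom.
; Each hole descent raises completion and reports it to the server through the MinigameState player state; debug inputs handle local connection and task-completion testing.
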(event CheckReadyStatus(NetworkController))

(event Custom|DragEvent1
  (params (Y%20Axis%20Delta :type Float%20%28single-precision%29))
  (bind _returnvalue (* Y%20Axis%20Delta 1.0))
  ;[1 1 1] Kameran Liikutus
  (Variables|Default|SetCameraCurrentHeight (.Z (Math|Vector|BreakVector (Transformation|GetActorLocation))))
  ;;[1 1 1] Onko kamera rajojen ulkopuolella
  (Math|Float|CompareFloat _returnvalue 0.0
    (:>
      (if (not (>= (Variables|Default|GetCameraCurrentHeight) (Variables|Default|GetCameraMaxHeight)))
        ;;[1 1 1] Kameran siirto
        (Transformation|AddActorWorldOffset (Math|Vector|MakeVector 0.0 0.0 _returnvalue) :!label _label)
        (Development|PrintString (Utilities|String|ToString(Float) _returnvalue))))
    (:<
      (if (not (<= (Variables|Default|GetCameraCurrentHeight) (Variables|Default|GetCameraMinHeight)))
        (goto _label)))))

(event Custom|SliderUpDown
  (params (ZoomPercent :type Float%20%28single-precision%29))
  (bind _camera (Variables|Default|GetCamera))
  ;[1 1 1] Kamera Zoom
  (Transformation|SetRelativeLocation _camera (* (Math|Vector|GetForwardVector _camera) (Math|Float|Lerp (Variables|Default|GetZoomMin) (Variables|Default|GetZoomMax) ZoomPercent)) false false))

(event Custom|GoDownHole
  ;[1 1 1] Robotin Liikutus alaspäin
  (Utilities|FlowControl|Delay 0.6)
  (Default|MoveDown (Variables|Default|GetRobo))
  (bind _asminigame_state (Utilities|Casting|CastToMinigameState (Variables|/Script/Engine.Controller|GetPlayerState (Game|GetPlayerController 0))))
  (bind _output_get (Variables|Default|Setcompletion (+ (Variables|Default|Getcompletion) (Variables|Default|GetCompletionIncrement))))
  (Class|MinigameState|ServerRPCTaskComplete _asminigame_state _output_get))

(event EventBeginPlay
  (bind _returnvalue (Transformation|GetActorLocation))
  (bind _returnvalue_2 (Game|GetPlayerController 0))
  (Variables|Default|SetHUDClass "/Game/Blueprints/UI/Widget/Minigame1_HUD.Minigame1_HUD_C")
  (Networking|SwitchHasAuthority
    (:Remote
      (Utilities|FlowControl|Sequence
        (:then_0
          ;[1 1 1] Spawn Gameboard
          (bind _returnvalue_3 (Game|SpawnActorfromClass "/Game/Blueprints/Level1/structure/structureBP.structureBP_C" (Math|Transform|MakeTransform (+ _returnvalue "600.000000,0.000000,-200.000000") "0,-90.000000, 0") "Undefined" 0 0))
          (Variables|Default|SetStructure _returnvalue_3)
          (Variables|Default|SetCameraMinHeight (.Z (Math|Vector|BreakVector _returnvalue)))
          (bind _returnvalue_4 (Actor|GetActorOfClass "/Game/Blueprints/Level1/Robot/RoboMovementBP.RoboMovementBP_C"))
          (Variables|Default|SetCameraMaxHeight (+ (.Z (Math|Vector|BreakVector (Transformation|GetActorLocation _returnvalue_4))) 2e+02))
          (Variables|/Script/Engine.PlayerController|SetbShowMouseCursor _returnvalue_2 true)
          (bind _asminigame_state (Utilities|Casting|CastToMinigameState (Variables|/Script/Engine.Controller|GetPlayerState _returnvalue_2)))
          (Class|MinigameState|ServerRPCTaskComplete _asminigame_state (Variables|Default|Getcompletion)))
        (:then_1
          ;[1 1 1] Kameran Liikutus
          (bind _returnvalue_5 (UserInterface|CreateWidget "/Game/Blueprints/Level1/widget/Touchwidget.Touchwidget_C"))
          (bind _output_get (Variables|Default|SetTouchWidget _returnvalue_5))
          (UserInterface|Viewport|AddtoViewport _output_get 0))
        (:then_2
          (EventDispatchers|BindEventtoOnDragUpDown (Variables|Default|GetTouchWidget) (delegate Custom|DragEvent1)))
        (:then_3
          ;[1 1 1] Kamera Zoom
          (EventDispatchers|BindEventtoOnSliderUpDown (Variables|Default|GetTouchWidget) (delegate Custom|SliderUpDown))
          (Variables|Default|SetZoomMin 0.0)
          (Variables|Default|SetZoomMax -1.2e+03))
        (:then_4
          ;[1 1 1] Robotin Liikutus alaspäin
          (EventDispatchers|BindEventtoGoDownHole (Variables|Default|GetRobo) (delegate Custom|GoDownHole)))))))

(event Collision|EventActorBeginOverlap
  (params (OtherActor :type Actor%20Object%20Reference)))

(event EventTick
  (params (DeltaSeconds :type Float%20%28single-precision%29)))

(event Input|ActionEvents|InputActionConnectionTest_Server
  (params (Key :type Key%20Structure :default "None")))

(event Input|ActionEvents|InputActionConnectionTest_Client
  (params (Key :type Key%20Structure :default "None"))
  (:Pressed
    (Development|ExecuteConsoleCommand "open 127.0.0.1" (Game|GetPlayerController 0))))

(event Input|ActionEvents|InputActionTestMap
  (params (Key :type Key%20Structure :default "None"))
  (:Pressed
    (bind _asminigame_playerstate (Utilities|Casting|CastToMinigame_Playerstate (Variables|/Script/Engine.Controller|GetPlayerState (Game|GetPlayerController 0))))
    (Class|MinigameState|ServerRPCTaskComplete _asminigame_playerstate 0.0)))

(event Input|KeyboardEvents|W
  (params (Key :type Key%20Structure :default "None"))
  (bind _robo (Variables|Default|GetRobo))
  (:Pressed
    (Networking|SwitchHasAuthority
      (:Remote
        (Utilities|IsValid _robo
          (:Is%20Valid
            (Default|MoveNorth _robo)))))))

(event Input|KeyboardEvents|S
  (params (Key :type Key%20Structure :default "None"))
  (bind _robo (Variables|Default|GetRobo))
  (:Pressed
    (Networking|SwitchHasAuthority
      (:Remote
        (Utilities|IsValid _robo
          (:Is%20Valid
            (Default|MoveSouth _robo)))))))

(event Input|KeyboardEvents|A
  (params (Key :type Key%20Structure :default "None"))
  (bind _robo (Variables|Default|GetRobo))
  (:Pressed
    (Networking|SwitchHasAuthority
      (:Remote
        (Utilities|IsValid _robo
          (:Is%20Valid
            (Default|MoveWest _robo)))))))

(event Input|KeyboardEvents|D
  (params (Key :type Key%20Structure :default "None"))
  (bind _robo (Variables|Default|GetRobo))
  (:Pressed
    (Networking|SwitchHasAuthority
      (:Remote
        (Utilities|IsValid _robo
          (:Is%20Valid
            (Default|MoveEast _robo)))))))

(event Input|KeyboardEvents|1
  (params (Key :type Key%20Structure :default "None"))
  (bind _structure (Variables|Default|GetStructure))
  (bind _stagearray (Variables|/Game/Blueprints/Level1/structure/structureBP.structureBP_C|GetStageArray _structure))
  (:Pressed
    (Networking|SwitchHasAuthority
      (:Remote
        (Utilities|IsValid _structure
          (:Is%20Valid
            (for (_array_element _array_index) _stagearray
              (if (== _array_index (/ (Utilities|Array|Length _stagearray) 2))
                (Default|Rotate _array_element)))))))))

(fn ConstructionScript)