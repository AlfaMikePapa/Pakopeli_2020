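; Robot actor for Level1 that moves in fixed steps in the four compass directions or downward.
; Each Move function sets a target location and facing, which Tick approaches with a swept constant-speed move and eased rotation.
; BeginPlay registers the robot with Game1Pawn and sets that pawn's camera height limit from the robot's height.
; Overlapping an actor whose name contains "floorwire" calls GoDownHole.
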(event OnComponentBeginOverlap(CollisionComponent)
  (params (OverlappedComponent :type Primitive%20Component%20Object%20Reference) (OtherActor :type Actor%20Object%20Reference) (OtherComp :type Primitive%20Component%20Object%20Reference) (OtherBodyIndex :type Integer) (bFromSweep :type Boolean) (SweepResult :type Hit%20Result%20Structure%20%28by%20ref%29))
  (if (Utilities|String|Contains (Utilities|GetDisplayName OtherActor) "floorwire")
    (Default|CallGoDownHole)))

(event EventBeginPlay
  (bind _asgame_1pawn (Utilities|Casting|CastToGame1Pawn (Game|Player|GetPlayerPawn 0)))
  (Variables|/Game/Blueprints/Level1/Game1Pawn.Game1Pawn_C|SetRobo _asgame_1pawn self)
  (Variables|/Game/Blueprints/Level1/Game1Pawn.Game1Pawn_C|SetCameraMaxHeight _asgame_1pawn (+ (.Z (Math|Vector|BreakVector (Transformation|GetActorLocation))) 1.5e+02)))

(event Collision|EventActorBeginOverlap
  (params (OtherActor :type Actor%20Object%20Reference)))

(event EventTick
  (params (DeltaSeconds :type Float%20%28single-precision%29))
  (if (not (and (Math|Vector|Equal(Vector) (Variables|Default|GetCurrentLocation) (Variables|Default|GetTargetLocation) 0.001) (Math|Rotator|Equal(Rotator) (Variables|Default|GetCurrentRotation) (Variables|Default|GetTargetRotation) 0.001)))
    (Utilities|FlowControl|Sequence
      (:then_0
        (Transformation|SetActorLocation (Math|Interpolation|VInterptoConstant (Variables|Default|GetCurrentLocation) (Variables|Default|GetTargetLocation) DeltaSeconds 1e+02) true false)
        (Variables|Default|SetCurrentLocation (Transformation|GetActorLocation)))
      (:then_1
        (Transformation|SetActorRotation (Math|Interpolation|RInterpTo (Variables|Default|GetCurrentRotation) (Variables|Default|GetTargetRotation) DeltaSeconds 8.0))
        (Variables|Default|SetCurrentRotation (Transformation|GetActorRotation))))))

(fn ConstructionScript)

(fn Move
  (params (MoveDirection :type Vector))
  (Variables|Default|SetCurrentRotation (Transformation|GetActorRotation))
  (bind _output_get (Variables|Default|SetCurrentLocation (Transformation|GetActorLocation)))
  (bind _output_get_2 (Variables|Default|SetTargetLocation (+ _output_get MoveDirection)))
  (Variables|Default|SetTargetRotation (Math|Rotator|FindLookatRotation _output_get _output_get_2)))

(fn MoveNorth
  (CallFunction|Move "100.000000, 0, 0"))

(fn MoveSouth
  (CallFunction|Move "-100.000000, 0, 0"))

(fn MoveEast
  (CallFunction|Move "0.000000,100.000000, 0"))

(fn MoveWest
  (CallFunction|Move "0.000000,-100.000000, 0"))

(fn MoveDown
  (CallFunction|Move "0.000000,0.000000,-130.000000"))