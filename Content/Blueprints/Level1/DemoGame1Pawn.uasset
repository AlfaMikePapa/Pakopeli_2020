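; Player pawn for a demo level that spawns the StructureBP gameboard, acts as the camera and steers the RoboMovementBP robot found in the level.
; WASD moves the robot in compass directions, and key 1 rotates the middle stage of the structure.
; A Touchwidget drives the camera: drags shift the pawn vertically within height limits, and a slider sets zoom.
; The robot's GoDownHole event triggers a delayed move down.
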(event Custom|DragEvent
  (params (Y%20Axis%20Delta :type Float%20%28single-precision%29))
  (bind _returnvalue (* Y%20Axis%20Delta 1.0))
  (Variables|Default|SetCameraCurrentHeight (.Z (Math|Vector|BreakVector (Transformation|GetActorLocation))))
  ;[1 1 1] Onko kamera rajojen ulkopuolella
  (Math|Float|CompareFloat _returnvalue 0.0
    (:>
      (if (not (>= (Variables|Default|GetCameraCurrentHeight) (Variables|Default|GetCameraMaxHeight)))
        ;[1 1 1] Kameran siirto
        (Transformation|AddActorWorldOffset (Math|Vector|MakeVector 0.0 0.0 _returnvalue) :!label _label)
        (Development|PrintString (Utilities|String|ToString(Float) _returnvalue))))
    (:<
      (if (not (<= (Variables|Default|GetCameraCurrentHeight) (Variables|Default|GetCameraMinHeight)))
        (goto _label)))))

(event Custom|SliderUpDown
  (params (ZoomPercent :type Float%20%28single-precision%29))
  (bind _cameracomponent (Variables|CameraActor|GetCameraComponent))
  ;[1 1 1] Kamera Zoom
  (Transformation|SetRelativeLocation _cameracomponent (* (Math|Vector|GetForwardVector _cameracomponent) (Math|Float|Lerp (Variables|Default|GetZoomMin) (Variables|Default|GetZoomMax) ZoomPercent)) false false))

(event Custom|GoDownHole
  (Utilities|FlowControl|Delay 0.6)
  (Default|MoveDown (Variables|Default|GetRobotti))
  (Development|PrintString "Hello"))

(event EventBeginPlay
  (bind _returnvalue (Transformation|GetActorLocation))
  (bind _returnvalue_2 (Game|GetPlayerController 0))
  (Utilities|FlowControl|Sequence
    (:then_0
      ;[1 1 1] Spawn Gameboard and set camera Heights
      (Input|EnableInput _returnvalue_2)
      (bind _returnvalue_3 (Game|SpawnActorfromClass "/Game/Blueprints/Level1/structure/structureBP.structureBP_C" (Math|Transform|MakeTransform (+ _returnvalue "600.000000,0.000000,-200.000000") "0,-90.000000, 0") "Undefined" 0 0))
      (Variables|Default|SetStructure _returnvalue_3)
      (Variables|Default|SetCameraMinHeight (.Z (Math|Vector|BreakVector _returnvalue)))
      (bind _returnvalue_4 (Actor|GetActorOfClass "/Game/Blueprints/Level1/Robot/RoboMovementBP.RoboMovementBP_C"))
      (bind _output_get (Variables|Default|SetRobotti _returnvalue_4))
      (Variables|Default|SetCameraMaxHeight (+ (.Z (Math|Vector|BreakVector (Transformation|GetActorLocation _output_get))) 2e+02))
      (Variables|/Script/Engine.PlayerController|SetbShowMouseCursor (Game|GetPlayerController 0) true))
    (:then_1
      (Game|Player|SetViewTargetwithBlend _returnvalue_2 self 0.0 "VTBlend_Linear" 0.0 false))
    (:then_2
      (bind _returnvalue_5 (UserInterface|CreateWidget "/Game/Blueprints/Level1/widget/Touchwidget.Touchwidget_C"))
      (bind _output_get_2 (Variables|Default|SetGUI _returnvalue_5))
      (UserInterface|Viewport|AddtoViewport _output_get_2 0))
    (:then_3
      (EventDispatchers|BindEventtoOnDragUpDown (Variables|Default|GetGUI) (delegate Custom|DragEvent)))
    (:then_4
      ;[1 1 1] Kamera Zoom
      (EventDispatchers|BindEventtoOnSliderUpDown (Variables|Default|GetGUI) (delegate Custom|SliderUpDown))
      (Variables|Default|SetZoomMin 0.0)
      (Variables|Default|SetZoomMax -1.2e+03))
    (:then_5
      (EventDispatchers|BindEventtoGoDownHole (Variables|Default|GetRobotti) (delegate Custom|GoDownHole)))))

(event Collision|EventActorBeginOverlap
  (params (OtherActor :type Actor%20Object%20Reference)))

(event EventTick
  (params (DeltaSeconds :type Float%20%28single-precision%29)))

(event Input|KeyboardEvents|W
  (params (Key :type Key%20Structure :default "None"))
  (:Pressed
    (Default|MoveNorth (Variables|Default|GetRobotti))))

(event Input|KeyboardEvents|S
  (params (Key :type Key%20Structure :default "None"))
  (:Pressed
    (Default|MoveSouth (Variables|Default|GetRobotti))))

(event Input|KeyboardEvents|A
  (params (Key :type Key%20Structure :default "None"))
  (:Pressed
    (Default|MoveWest (Variables|Default|GetRobotti))))

(event Input|KeyboardEvents|D
  (params (Key :type Key%20Structure :default "None"))
  (:Pressed
    (Default|MoveEast (Variables|Default|GetRobotti))))

(event Input|KeyboardEvents|1
  (params (Key :type Key%20Structure :default "None"))
  (bind _structure (Variables|Default|GetStructure))
  (bind _stagearray (Variables|/Game/Blueprints/Level1/structure/structureBP.structureBP_C|GetStageArray _structure))
  (:Pressed
    (for (_array_element _array_index) _stagearray
      (if (== _array_index (/ (Utilities|Array|Length _stagearray) 2))
        (Default|Rotate _array_element)))))

(fn ConstructionScript)