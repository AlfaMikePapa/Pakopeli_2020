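; Level 1 floor tile Blueprint whose emissive glow reacts to anything overlapping its Box trigger.
; Overlap start targets green and briefly spikes brightness before settling lower; overlap end targets yellow at a slower blend speed.
; Tick eases colour and brightness toward their targets, writing them to the FloorTile material parameters and skipping work once both are nearly equal.
; The construction script initialises the emission to white.
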(event OnComponentBeginOverlap(Box)
  (params (OverlappedComponent :type Primitive%20Component%20Object%20Reference) (OtherActor :type Actor%20Object%20Reference) (OtherComp :type Primitive%20Component%20Object%20Reference) (OtherBodyIndex :type Integer) (bFromSweep :type Boolean) (SweepResult :type Hit%20Result%20Structure%20%28by%20ref%29))
  ;[1 1 1] SetColourTargetGreen
  (Variables|Default|SetColourTarget (Utilities|Struct|MakeLinearColor 0.0 1.0 0.0 0.0))
  (Variables|Default|SetInterpolationSpeed 3.0)
  ;[1 1 1] Set Brightness Target, Flash
  (Variables|Default|SetBrightnessTarget 1.09e+03)
  (Utilities|FlowControl|Delay 0.1)
  (Variables|Default|SetBrightnessTarget 3e+01))

(event OnComponentEndOverlap(Box)
  (params (OverlappedComponent :type Primitive%20Component%20Object%20Reference) (OtherActor :type Actor%20Object%20Reference) (OtherComp :type Primitive%20Component%20Object%20Reference) (OtherBodyIndex :type Integer))
  ;[1 1 1] SetColourTargetYellow
  (Variables|Default|SetColourTarget (Utilities|Struct|MakeLinearColor 1.0 1.0 0.0 0.0))
  (Variables|Default|SetInterpolationSpeed 0.5))

(event EventBeginPlay)

(event Collision|EventActorBeginOverlap
  (params (OtherActor :type Actor%20Object%20Reference)))

(event EventTick
  (params (DeltaSeconds :type Float%20%28single-precision%29))
  ;[1 1 1] Check if anything needs interpolating
  (if (not (and (Class|KismetMathLibrary|LinearColorIsNearEqual (Variables|Default|GetColourCurrent) (Variables|Default|GetColourTarget) 0.01) (Math|Float|NearlyEqual(Float) (Variables|Default|GetBrightnessTarget) (Variables|Default|GetBrightnessCurrent) 0.01)))
    ;[1 1 1] Interpolate Colour
    (Rendering|Material|SetVectorParameterValueonMaterials (Variables|Default|GetFloorTile) "EmissionColour" (Math|Conversions|ToVector(LinearColor) (Class|KismetMathLibrary|CInterpto (Variables|Default|GetColourCurrent) (Variables|Default|GetColourTarget) DeltaSeconds (Variables|Default|GetInterpolationSpeed))))
    (Variables|Default|SetColourCurrent (Class|KismetMathLibrary|CInterpto (Variables|Default|GetColourCurrent) (Variables|Default|GetColourTarget) DeltaSeconds (Variables|Default|GetInterpolationSpeed)))
    ;[1 1 1] InterpolateBrightness
    (Rendering|Material|SetScalarParameterValueonMaterials (Variables|Default|GetFloorTile) "EmissionStrength" (Math|Interpolation|FInterpTo (Variables|Default|GetBrightnessCurrent) (Variables|Default|GetBrightnessTarget) DeltaSeconds 8.0))
    (Variables|Default|SetBrightnessCurrent (Math|Interpolation|FInterpTo (Variables|Default|GetBrightnessCurrent) (Variables|Default|GetBrightnessTarget) DeltaSeconds 8.0))))

(fn ConstructionScript
  (Rendering|Material|CreateDynamicMaterialInstance "/Game/Assets/level1/materials/structure/level1_material.level1_material" "None" :!class /Script/Engine.KismetMaterialLibrary)
  (bind _output_get (Variables|Default|SetColourCurrent (Utilities|Struct|MakeLinearColor 1.0 1.0 1.0 0.0)))
  (Rendering|Material|SetVectorParameterValueonMaterials (Variables|Default|GetFloorTile) "EmissionColour" (Math|Conversions|ToVector(LinearColor) _output_get))
  (Rendering|Material|SetScalarParameterValueonMaterials (Variables|Default|GetFloorTile) "EmissionStrength" 5e+01))