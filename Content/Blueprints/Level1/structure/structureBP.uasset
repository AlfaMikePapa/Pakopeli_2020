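; Level 1 structure actor that builds a vertical stack of stages at BeginPlay for a minigame, sized by the difficulty level in the player state.
; Difficulty sets the stage count, from which Game1Pawn receives its per-stage completion increment.
; A countdown loop adds stageBP child actors at stepped heights from the top down, storing them in StageArray.
; RoboMovementBP then spawns just above the first stored stage, the topmost one.
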(event EventBeginPlay
  (Utilities|FlowControl|Sequence
    (:then_0
      (bind _asminigame_playerstate (Utilities|Casting|CastToMinigame_Playerstate (Variables|/Script/Engine.Controller|GetPlayerState (Game|GetPlayerController 0))))
      (Development|PrintString (Utilities|String|ToString(Integer) (Variables|/Game/Blueprints/Server/Minigame_Playerstate.Minigame_Playerstate_C|GetDifficultyLevel _asminigame_playerstate)))
      (switch int (Variables|/Game/Blueprints/Server/Minigame_Playerstate.Minigame_Playerstate_C|GetDifficultyLevel _asminigame_playerstate)
        (:0
          (Variables|Default|Setloopcount 2))
        (:1
          (Variables|Default|Setloopcount 3))
        (:2
          (Variables|Default|Setloopcount 5))
        (:3
          (Variables|Default|Setloopcount 60)))
      (bind _asgame_1pawn (Utilities|Casting|CastToGame1Pawn (Game|Player|GetPlayerPawn 0)))
      (Variables|/Game/Blueprints/Level1/Game1Pawn.Game1Pawn_C|SetCompletionIncrement _asgame_1pawn (/ 1.0 (Math|Conversions|ToFloat(Integer) (+ (Variables|Default|Getloopcount) 1)))))
    (:then_1
      (while (>= (Variables|Default|Getloopcount) 0)
        ;[1 1 1] ConstructionLoop
        (bind _returnvalue (AddComponent|AddChildActorComponent false (Math|Transform|MakeTransform (Math|Vector|MakeVector 0.0 0.0 (Math|Conversions|ToFloat(Integer) (* (Variables|Default|GetTransformZ) (Variables|Default|Getloopcount)))))))
        (bind _result (Math|Integer|DecrementInt (Variables|Default|Getloopcount))
          (:%20%20
            (Variables|Default|Setloopcount _result)
            (bind _asstage_bp (Utilities|Casting|CastTostageBP (Variables|/Script/Engine.ChildActorComponent|GetChildActor _returnvalue)))
            (Utilities|Array|Add (Variables|Default|GetStageArray) _asstage_bp)))))
    (:then_2
      (bind _stagetransform (Default|GetStageTransform (Utilities|Array|Get(acopy) (Variables|Default|GetStageArray))))
      (Game|SpawnActorfromClass "/Game/Blueprints/Level1/Robot/RoboMovementBP.RoboMovementBP_C" (Math|Transform|MakeTransform (+ (.Location (Math|Transform|BreakTransform _stagetransform)) "0, 0,38.000000")) "Undefined" 0 0))))

(event Collision|EventActorBeginOverlap
  (params (OtherActor :type Actor%20Object%20Reference)))

(event EventTick
  (params (DeltaSeconds :type Float%20%28single-precision%29)))

(fn ConstructionScript)