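; Stage actor for Level 1 that builds a tiled floor with one random hole and rotates in 90-degree steps.
; The construction script spawns child actors at listed tile coordinates, using a floorwireBP at the randomly picked hole index and keeping a reference to it.
; Pressing Z sets a new target rotation, which Tick approaches at constant speed with RInterpToConstant.
; GetStageTransform exposes the actor's transform.
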(event EventBeginPlay
  (Input|EnableInput (Game|GetPlayerController 0)))

(event Collision|EventActorBeginOverlap
  (params (OtherActor :type Actor%20Object%20Reference)))

(event EventTick
  (params (DeltaSeconds :type Float%20%28single-precision%29))
  (if (not (Math|Rotator|Equal(Rotator) (Variables|Default|GetCurrentRotation) (Variables|Default|GetTargetRotation) 0.01))
    (Transformation|SetActorRotation (Class|KismetMathLibrary|RInterptoConstant (Variables|Default|GetCurrentRotation) (Variables|Default|GetTargetRotation) DeltaSeconds 1e+02))
    (Variables|Default|SetCurrentRotation (Transformation|GetActorRotation))))

(event Input|KeyboardEvents|Z
  (params (Key :type Key%20Structure :default "None"))
  (:Pressed
    (CallFunction|Rotate)))

(fn ConstructionScript
  (Utilities|FlowControl|Sequence
    (:then_0
      ;[1 1 1] Generate Hole Location
      (Variables|Default|SetRandom (Math|Random|RandomInteger 8)))
    (:then_1
      ;[1 1 1] Generate the Stage
      (for (_array_element _array_index) (Variables|Default|GetFloortileCoordinateList)
        (Utilities|Array|Add (Variables|Default|GetHoleLocationArray) (Variables|Default|GetRandom))
        (if (== _array_index (Variables|Default|GetRandom))
          ;;[1 1 1] Hole
          (bind _returnvalue (AddComponent|AddChildActorComponent false (Math|Transform|MakeTransform (Math|Vector|MakeVector (.X (Math|Vector|BreakVector _array_element)) (.Y (Math|Vector|BreakVector _array_element)) 0.0))))
          (bind _asfloorwire_bp (Utilities|Casting|CastTofloorwireBP (Variables|/Script/Engine.ChildActorComponent|GetChildActor _returnvalue)))
          (Variables|Default|SetFloorWire _asfloorwire_bp)
          (else
            ;;[1 1 1] Floorpiece
            (AddComponent|AddChildActorComponent false (Math|Transform|MakeTransform (Math|Vector|MakeVector (.X (Math|Vector|BreakVector _array_element)) (.Y (Math|Vector|BreakVector _array_element)) 0.0)))))))))

(fn Rotate
  (bind _output_get (Variables|Default|SetCurrentRotation (Transformation|GetActorRotation)))
  (Variables|Default|SetTargetRotation (Math|Rotator|CombineRotators _output_get "0,90.000000, 0")))

(fn GetStageTransform
  (return (Transformation|GetActorTransform)))