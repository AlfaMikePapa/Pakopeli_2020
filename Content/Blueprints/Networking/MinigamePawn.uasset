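; MinigamePawn is a pawn, apparently a base for minigames, that supplies a function to set up the on-screen HUD.
; InitializeHUD skips setup when HUDClass is Minigame1_HUD; otherwise it creates the widget for player controller 0, adds it to the viewport and shows the mouse cursor.
; An invalid class prints a "NO HUD!" warning.
; The event graph is empty, and nothing in this file calls InitializeHUD.
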(event EventBeginPlay)

(event Collision|EventActorBeginOverlap
  (params (OtherActor :type Actor%20Object%20Reference)))

(event EventTick
  (params (DeltaSeconds :type Float%20%28single-precision%29)))

(fn ConstructionScript)

(fn InitializeHUD
  (bind _returnvalue (Game|GetPlayerController 0))
  (bind _hudclass (Variables|Default|GetHUDClass))
  (if (!= (Variables|Default|GetHUDClass) "/Game/Blueprints/UI/Widget/Minigame1_HUD.Minigame1_HUD_C")
    (if (Utilities|IsValidClass _hudclass)
      (bind _returnvalue_2 (UserInterface|CreateWidget _hudclass _returnvalue))
      (bind _output_get (Variables|Default|SetHUD _returnvalue_2))
      (UserInterface|Viewport|AddtoViewport _output_get 0)
      (Variables|/Script/Engine.PlayerController|SetbShowMouseCursor _returnvalue true)
      (else
        (Development|PrintString "NO HUD!" true true "(R=0.343750,G=0.000000,B=0.005089,A=1.000000)")))))