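; Player state for a networked escape game that links each client's minigame to the server's HUD and Escape_Gamemode.
; On the server it takes difficulty from the game mode; on clients it loads the game type from a save and sends it by RPC.
; Bound events initialize the client pawn's HUD, update readiness and progress on the server HUD, and notify the game mode of setup and task completion.
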(event Custom|MarkTaskComplete
  ;[1 1 1] When client reports task complete
  (bind _asescape_gamemode (Utilities|Casting|CastToEscape_Gamemode (Game|GetGameMode)))
  (Default|TaskCompleted _asescape_gamemode (Variables|Default|GetControlledGame))
  (Variables|Default|SetbIsCompleted true)
  (bind _asserver_pawn (Utilities|Casting|CastToServerPawn (Pawn|GetControlledPawn (Game|GetPlayerController 0))))
  (if (Utilities|IsValid (Variables|/Game/Blueprints/Server/ServerPawn.ServerPawn_C|GetHUD _asserver_pawn))
    (switch Utilities|FlowControl|Switch|SwitchonEGameType (Variables|Default|GetControlledGame_0)
      (:Minigame1
        (Default|SetTask1Complete (Variables|/Game/Blueprints/Server/ServerPawn.ServerPawn_C|GetHUD _asserver_pawn)))
      (:Minigame2
        (Default|SetTask2Complete (Variables|/Game/Blueprints/Server/ServerPawn.ServerPawn_C|GetHUD _asserver_pawn)))
      (:Minigame3
        (Default|SetTask3Complete (Variables|/Game/Blueprints/Server/ServerPawn.ServerPawn_C|GetHUD _asserver_pawn))))))

(event Custom|ConfirmConnection
  (Variables|Default|SetbIsConnected true))

(event Custom|SetConnection
  (params (HUD :type Minigame%20HUD%20Object%20Reference))
  (Default|SetConnectionStatus HUD (Variables|Default|GetbIsConnected)))

(event Custom|SetClientReady
  (bind _isreadytostart (Variables|Default|GetIsReadyToStart))
  (bind _serverhud (Variables|Default|GetServerHUD))
  ;[1 1 1] Update client ready status
  (Utilities|IsValid _serverhud
    (:Is%20Valid
      (switch Utilities|FlowControl|Switch|SwitchonEGameType (Variables|Default|GetControlledGame_0)
        (:Minigame1
          (Default|SetTask1Ready _serverhud _isreadytostart))
        (:Minigame2
          (Default|SetTask2Ready _serverhud _isreadytostart))
        (:Minigame3
          (Default|SetTask3Ready _serverhud _isreadytostart))))))

(event Custom|ReadyToInitialize
  ;[1 1 1] Setup Complete
  (Development|PrintString "Ready to go" true true "(R=1.000000,G=0.173728,B=0.949183,A=1.000000)")
  (Development|PrintString (Utilities|String|EnumtoString (Variables|Default|GetControlledGame)) true true "(R=0.189640,G=1.000000,B=0.000000,A=1.000000)")
  (bind _asescape_gamemode (Utilities|Casting|CastToEscape_Gamemode (Game|GetGameMode)))
  (Default|InitializePawn _asescape_gamemode))

(event Custom|Update%20Task%20Status
  ;[1 1 1] On Task Status Update Received
  (Default|SetTaskProgress (Variables|Default|GetServerHUD) (Variables|Default|GetControlledGame) (Variables|Default|GetTaskCompletionRate)))

(event Custom|InitializeHUD
  (bind _returnvalue (Game|GetPlayerController 0))
  (bind _returnvalue_2 (Pawn|GetControlledPawn _returnvalue))
  ;[1 1 1] Create HUD on the client
  (Utilities|IsValid _returnvalue_2
    (:Is%20Valid
      (bind _asminigame_pawn (Utilities|Casting|CastToMinigamePawn _returnvalue_2))
      (Default|InitializeHUD _asminigame_pawn))))

(event EventBeginPlay
  (Utilities|FlowControl|Sequence
    (:then_0
      (Networking|SwitchHasAuthority
        (:Authority
          (bind _asserver_pawn (Utilities|Casting|CastToServerPawn (Pawn|GetControlledPawn (Game|GetPlayerController 0))))
          (Utilities|FlowControl|Sequence
            (:then_0
              (bind _asescape_gamemode (Utilities|Casting|CastToEscape_Gamemode (Game|GetGameMode)))
              (Development|PrintString (Utilities|String|ToString(Integer) (Variables|/Game/Blueprints/Server/Escape_Gamemode.Escape_Gamemode_C|GetDifficultyLevel _asescape_gamemode)))
              (Variables|Default|SetDifficultyLevel (Variables|/Game/Blueprints/Server/Escape_Gamemode.Escape_Gamemode_C|GetDifficultyLevel _asescape_gamemode)))
            (:then_1
              (if (Utilities|IsValid (Variables|/Game/Blueprints/Server/ServerPawn.ServerPawn_C|GetHUD _asserver_pawn))
                (Variables|Default|SetServerHUD (Variables|/Game/Blueprints/Server/ServerPawn.ServerPawn_C|GetHUD _asserver_pawn))
                (Variables|Default|SetControlledGame "GameServer")))))
        (:Remote
          (CallFunction|LoadGameType))))
    (:then_1
      ;[1 1 1] Bind events
      (EventDispatchers|BindEventtoClientConnected (delegate Custom|SetClientReady))
      (EventDispatchers|BindEventtoClientReadyUp (delegate Custom|SetClientReady))
      (EventDispatchers|BindEventtoInitializeClientHUD (delegate Custom|InitializeHUD))
      (EventDispatchers|BindEventtoTaskComplete (delegate Custom|MarkTaskComplete))
      (EventDispatchers|BindEventtoSetupComplete (delegate Custom|ReadyToInitialize))
      (EventDispatchers|BindEventtoTaskStatusUpdate (delegate Custom|Update%20Task%20Status)))))

(event EventTick
  (params (DeltaSeconds :type Float%20%28single-precision%29)))

(fn ConstructionScript
  (Networking|SwitchHasAuthority
    (:Remote
      (Development|PrintString "Hello"))))

(fn LoadGameType
  (bind _returnvalue (SaveGame|DoesSaveGameExist "ClientOptions"))
  (if _returnvalue
    (bind _returnvalue_2 (SaveGame|LoadGamefromSlot "ClientOptions"))
    (bind _assave_client_options (Utilities|Casting|CastToSaveClientOptions _returnvalue_2))
    (bind _output_get (Variables|Default|SetControlledGame (Variables|/Game/Blueprints/Saving/SaveClientOptions.SaveClientOptions_C|GetGameType _assave_client_options)))
    (Class|MinigameState|ServerRPCInboundSettings _output_get)
    (else
      (Development|PrintString "No Save file" true true "(R=0.411458,G=0.012766,B=0.020952,A=1.000000)"))))