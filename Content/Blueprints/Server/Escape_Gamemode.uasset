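; Game mode for a multiplayer escape game that pairs a server player with clients playing three minigames.
; The first login becomes the server; later logins read their game from Minigame_Playerstate, which selects the pawn class.
; On restart it confirms the connection, teleports the pawn to its named PlayerStart and initializes the HUD by client RPC.
; TaskCompleted records finished minigames, but only games 2 and 3 are required to show the server's completion HUD.
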(event Custom|TaskCompleted
  (params (Game :type EGameType%20Enum :default "None"))
  (switch Utilities|FlowControl|Switch|SwitchonEGameType Game
    (:Minigame1
      (Variables|Default|SetGame1Complete true))
    (:Minigame2
      (Variables|Default|SetGame2Complete true))
    (:Minigame3
      (Variables|Default|SetGame3Complete true)))
  (CallFunction|CheckGameStatus))

(event EventBeginPlay
  (Variables|Default|SetServerPlayerController (Game|GetPlayerController 0)))

(event EventTick
  (params (DeltaSeconds :type Float%20%28single-precision%29)))

(event EventPostLogin
  (params (NewPlayer :type Player%20Controller%20Object%20Reference))
  (bind _playercontrollers (Variables|Default|GetPlayerControllers))
  (Utilities|Array|AddUnique _playercontrollers NewPlayer)
  (if (== (Utilities|Array|Length _playercontrollers) 1)
    (Variables|Default|SetLastGameType "GameServer")
    (else
      (bind _asminigame_playerstate (Utilities|Casting|CastToMinigame_Playerstate (Variables|/Script/Engine.Controller|GetPlayerState NewPlayer)))
      (bind _output_get (Variables|Default|SetLastGameType (Variables|/Game/Blueprints/Server/Minigame_Playerstate.Minigame_Playerstate_C|GetControlledGame_0 _asminigame_playerstate)))
      (Development|PrintString (Utilities|String|EnumtoString _output_get) true true "(R=0.906830,G=0.958749,B=1.000000,A=1.000000)" 2e+02)))
  (Class|GameModeBase|RestartPlayer NewPlayer))

(event EventOnLogout
  (params (ExitingController :type Controller%20Object%20Reference))
  (bind _asplayer_controller (Utilities|Casting|CastToPlayerController ExitingController))
  (Utilities|Array|RemoveItem (Variables|Default|GetPlayerControllers) _asplayer_controller))

(event EventOnRestartPlayer
  (params (NewPlayer :type Controller%20Object%20Reference))
  (CallFunction|OnPawnInitialized NewPlayer NewPlayer))

(fn ConstructionScript)

(fn ChoosePlayerStart
  (params (Player :type Controller%20Object%20Reference))
  (return (Class|GameModeBase|FindPlayerStart Player "None")))

(fn GetNextGameType
  (if true
    (switch Utilities|FlowControl|Switch|SwitchonEGameType (Variables|Default|GetLastGameType)
      (:None
        (Variables|Default|SetLastGameType "GameServer"))
      (:Minigame1
        (Variables|Default|SetLastGameType "Minigame2"))
      (:Minigame2
        (Variables|Default|SetLastGameType "Minigame3"))
      (:GameServer
        (Variables|Default|SetLastGameType "Minigame1")))))

(fn GetDefaultPawnClassforController
  (params (InController :type Controller%20Object%20Reference))
  (switch Utilities|FlowControl|Switch|SwitchonEGameType (Variables|Default|GetLastGameType)
    (:None
      (return "/Script/Engine.DefaultPawn"))
    (:Minigame1
      (return "/Game/Blueprints/Level1/Game1Pawn.Game1Pawn_C"))
    (:Minigame2
      (return "/Game/Blueprints/Level2/Game2Pawn_BP.Game2Pawn_BP_C"))
    (:Minigame3
      (return "/Game/Blueprints/Level3/Game3Pawn_BP.Game3Pawn_BP_C"))
    (:GameServer
      (bind _returnvalue (|CallParentFunction 0))
      (return _returnvalue))))

(fn InitializePawn
  (bind _playercontrollers (Variables|Default|GetPlayerControllers))
  (bind _returnvalue (Utilities|Array|LastIndex _playercontrollers))
  (bind _output (Utilities|Array|Get(acopy) _playercontrollers _returnvalue))
  (bind _asminigame_playerstate (Utilities|Casting|CastToMinigame_Playerstate (Variables|/Script/Engine.Controller|GetPlayerState _output)))
  (Development|PrintString (Utilities|String|EnumtoString (Variables|/Script/Pakopeli_2020.MinigameState|GetControlledGame _asminigame_playerstate)) true true "(R=1.000000,G=0.980391,B=0.097830,A=1.000000)" 222.0)
  (bind _output_get (Variables|Default|SetLastGameType (Variables|/Script/Pakopeli_2020.MinigameState|GetControlledGame _asminigame_playerstate)))
  (switch Utilities|FlowControl|Switch|SwitchonEGameType _output_get
    (:Minigame1
      (bind _returnvalue_2 (Game|SpawnActorfromClass "/Game/Blueprints/Level1/Game1Pawn.Game1Pawn_C" (Transformation|GetActorTransform (Class|GameModeBase|FindPlayerStart 0 "Minigame1")) "Undefined" 0 0))
      (Pawn|Possess _output _returnvalue_2))
    (:Minigame2
      (bind _returnvalue_3 (Game|SpawnActorfromClass "/Game/Blueprints/Level2/Game2Pawn_BP.Game2Pawn_BP_C" (Transformation|GetActorTransform (Class|GameModeBase|FindPlayerStart 0 "Minigame2")) "Undefined" 0 0))
      (Pawn|Possess _output _returnvalue_3))
    (:Minigame3
      (bind _returnvalue_4 (Game|SpawnActorfromClass "/Game/Blueprints/Level3/Game3Pawn_BP.Game3Pawn_BP_C" (Transformation|GetActorTransform (Class|GameModeBase|FindPlayerStart 0 "Minigame3")) "Undefined" 0 0))
      (Pawn|Possess _output _returnvalue_4)))
  (CallFunction|OnPawnInitialized 0 _output)
  (Variables|Default|SetLastGameType "None"))

(fn OnPawnInitialized
  (params (self2 :type Controller%20Object%20Reference) (Controller :type Controller%20Object%20Reference))
  (bind _asminigame_playerstate (Utilities|Casting|CastToMinigame_Playerstate (Variables|/Script/Engine.Controller|GetPlayerState Controller)))
  (Variables|/Game/Blueprints/Server/Minigame_Playerstate.Minigame_Playerstate_C|SetControlledGame_0 _asminigame_playerstate (Variables|Default|GetLastGameType))
  (Default|ConfirmConnection _asminigame_playerstate)
  (Class|MinigameState|ServerRPCClientConnected _asminigame_playerstate)
  (switch Utilities|FlowControl|Switch|SwitchonEGameType (Variables|/Game/Blueprints/Server/Minigame_Playerstate.Minigame_Playerstate_C|GetControlledGame_0 _asminigame_playerstate)
    (:Minigame1
      (Variables|Default|SetStartToFind "Minigame1"))
    (:Minigame2
      (Variables|Default|SetStartToFind "Minigame2"))
    (:Minigame3
      (Variables|Default|SetStartToFind "Minigame3"))
    (:GameServer
      (Variables|Default|SetStartToFind "None")))
  (Transformation|SetActorTransform (Pawn|GetControlledPawn Controller) (Transformation|GetActorTransform (Class|GameModeBase|FindPlayerStart Controller (Variables|Default|GetStartToFind))) false true)
  (Class|MinigameState|ClientRPCInitializeHUD _asminigame_playerstate))

(fn CheckGameStatus
  (if (and (Variables|Default|GetGame2Complete) (Variables|Default|GetGame3Complete))
    (CallFunction|GameComplete)))

(fn GameComplete
  (bind _asserver_pawn (Utilities|Casting|CastToServerPawn (Game|Player|GetPlayerPawn 0)))
  (Default|ShowCompleteElements (Variables|/Game/Blueprints/Server/ServerPawn.ServerPawn_C|GetHUD _asserver_pawn) true))