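; Player controller for Level2 that holds a slot-based inventory in an InventoryObjects array.
; InventoryCheck and FindEmptySlot scan for invalid entries, and MoveItem moves or swaps items, though its swap writes to the default index instead of the target slot.
; PickUpItem and MoveImage contain disconnected logic for storing items and updating HUD button images, so neither does anything.
; RemoveItem and ItemWasUsed are empty stubs.
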(event EventBeginPlay)

(fn ConstructionScript)

(fn InventoryCheck
  (for _array_element (Variables|Default|GetInventoryObjects)
    (if (not (Utilities|IsValid _array_element))
      (LocalVariables|SetSpacesAvailable (+ (LocalVariables|GetSpacesAvailable) 1))))
  (if (> (LocalVariables|GetSpacesAvailable) 0)
    (Variables|Default|SetHasInventorySpace? true)
    (else
      (Variables|Default|SetHasInventorySpace? false)))
  (return (Variables|Default|GetHasInventorySpace?)))

(fn PickUpItem
  (params (ItemToPickup :type Object%20Object%20Reference)))

(fn FindEmptySlot
  (bind (_array_element _array_index) (Utilities|Array|ForEachLoopwithBreak (Variables|Default|GetInventoryObjects) :!label _label)
    (:LoopBody
      (if (not (Utilities|IsValid _array_element))
        (bind _output_get (Variables|Default|SetEmptySlot _array_index))
        (goto _label Break)))
    (:Completed
      (return _output_get))))

(fn MoveItem
  (params (From :type Integer) (To :type Integer))
  (bind _inventoryobjects (Variables|Default|GetInventoryObjects))
  (bind _inventoryobjects_2 (Variables|Default|GetInventoryObjects))
  (LocalVariables|SetLocalFrom From)
  (LocalVariables|SetLocalTo To)
  (if (Utilities|IsValid (Utilities|Array|Get(acopy) (Variables|Default|GetInventoryObjects) (LocalVariables|GetLocalTo)))
    (LocalVariables|SetLocalTempObject (Utilities|Array|Get(acopy) (Variables|Default|GetInventoryObjects) (LocalVariables|GetLocalTo)))
    (Utilities|Array|SetArrayElem _inventoryobjects 0 (Utilities|Array|Get(acopy) _inventoryobjects (LocalVariables|GetLocalFrom)))
    (Utilities|Array|SetArrayElem (Variables|Default|GetInventoryObjects) (LocalVariables|GetLocalFrom) (LocalVariables|GetLocalTempObject))
    (LocalVariables|SetLocalSwapping? true)
    (else
      (Utilities|Array|SetArrayElem _inventoryobjects_2 (LocalVariables|GetLocalTo) (Utilities|Array|Get(acopy) _inventoryobjects_2 (LocalVariables|GetLocalFrom)))
      (Utilities|Array|SetArrayElem (Variables|Default|GetInventoryObjects) (LocalVariables|GetLocalFrom) 0)
      (LocalVariables|SetLocalSwapping? false)))
  (return (LocalVariables|GetLocalSwapping?)))

(fn MoveImage
  (params (From :type Integer) (To :type Integer) (ItemImage :type Texture%202D%20Object%20Reference) (Swapping :type Boolean)))

(fn RemoveItem
  (params (InventorySlot :type Integer) (ActionSlot :type Integer) (PickupItemImage :type Texture%202D%20Object%20Reference)))

(fn ItemWasUsed
  (params (SlotUsed :type Integer)))