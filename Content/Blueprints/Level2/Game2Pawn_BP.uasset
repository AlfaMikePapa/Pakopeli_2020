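; Player pawn for the networked Level 2 minigame that runs the puzzle gameboard and reports progress to the server.
; On BeginPlay the remote client's local pawn sets up the HUD, spawns a Gameboard scaled to the PlayerState difficulty and angles the camera.
; ExecuteMoves passes queued moves to the board, while UpdateGameState sends progress through a PlayerState server RPC.
; A debug input connects to localhost, and some goal-generation test nodes are left unconnected.
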(event CheckReadyStatus(NetworkController))

(event EventBeginPlay
  ;[1 1 1] Updates game state to reflect a started game
  (Variables|Default|SetHUDClass "/Game/Blueprints/UI/Widget/Minigame2_HUD.Minigame2_HUD_C")
  (if (== self (Game|Player|GetPlayerPawn 0))
    (CallFunction|UpdateGameState (Variables|Default|GetGameState))
    (Utilities|Casting|CastToMinigame_Playerstate (Variables|Default|GetPlayerState))
    ;[1 1 1] Spawns Gameboard with the proper difficulty and sets camera to the correct orientation, and sets reference to it for hud
    (Networking|SwitchHasAuthority
      (:Remote
        (CallFunction|InitializeHUD)
        (bind _returnvalue (Game|SpawnActorfromClass "/Game/Game2BP/Blueprints/Gameboard.Gameboard_C" (Math|Transform|MakeTransform (Math|Vector|MakeVector 0.0 -2.8e+02 0.0) (Math|Rotator|MakeRotator 0.0 0.0 9e+01)) "Undefined" 0 0))
        (bind _asminigame_2_hud (Utilities|Casting|CastToMinigame2_HUD (Variables|Default|GetHUD)))
        (Default|SetGameBoardReference _asminigame_2_hud _returnvalue)
        (bind _output_get (Variables|Default|SetGameboard _returnvalue))
        (bind _asminigame_playerstate (Utilities|Casting|CastToMinigame_Playerstate (Variables|/Script/Engine.Controller|GetPlayerState (Game|GetPlayerController 0)))
          (:then
            (if (.ReturnValue (Utilities|Map|Find (Variables|Default|GetDifficultyMap) (Variables|/Game/Blueprints/Server/Minigame_Playerstate.Minigame_Playerstate_C|GetDifficultyLevel _asminigame_playerstate)))
              (Default|SpawnEvent _output_get (.Value (Utilities|Map|Find (Variables|Default|GetDifficultyMap) (Variables|/Game/Blueprints/Server/Minigame_Playerstate.Minigame_Playerstate_C|GetDifficultyLevel _asminigame_playerstate))))
              (else
                (Default|SpawnEvent _output_get 5)))
            (Pawn|SetControlRotation (Pawn|GetController self) (Math|Rotator|MakeRotator 0.0 -8e+01 -9e+01))
            (Utilities|Casting|CastToMinigame_Playerstate (Variables|/Script/Engine.Controller|GetPlayerState (Game|GetPlayerController 0))))
          (:CastFailed
            (Development|PrintString "Cast to Game2 Playerstate failed!")))))))

(event Collision|EventActorBeginOverlap
  (params (OtherActor :type Actor%20Object%20Reference)))

(event EventTick
  (params (DeltaSeconds :type Float%20%28single-precision%29)))

(event Input|ActionEvents|InputActionConnectionTest_Server
  (params (Key :type Key%20Structure :default "None")))

(event Input|ActionEvents|InputActionConnectionTest_Client
  (params (Key :type Key%20Structure :default "None"))
  (:Pressed
    (Development|ExecuteConsoleCommand "open 127.0.0.1" (Game|GetPlayerController 0))))

(fn ConstructionScript)

(fn UpdateGameState
  (params (NewGameState :type Float%20%28single-precision%29))
  ;[1 1 1] Sends game progress to the server via PlayerState. Progress 0.0-1.0 (corresponds to a percentage)
  (Networking|SwitchHasAuthority
    (:Remote
      (bind _asminigame_playerstate (Utilities|Casting|CastToMinigame_Playerstate (Variables|/Script/Engine.Controller|GetPlayerState (Game|GetPlayerController 0))))
      (bind _output_get (Variables|Default|SetGameState NewGameState))
      (Class|MinigameState|ServerRPCTaskComplete _asminigame_playerstate _output_get))))

(fn ExecuteMoves
  (params (MoveQueue :type Array%20of%20Integers))
  ;[1 1 1] Sends queued moves to Gameboard and updates gamestate to corresponding value for server
  (Networking|SwitchHasAuthority
    (:Remote
      (CallFunction|UpdateGameState 0.5)
      (Default|ExecuteMoves (Variables|Default|GetGameboard) MoveQueue))))