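; Clickable cable connection in the Level 3 energy path puzzle, shown according to difficulty level.
; On BeginPlay it stretches an InputHandler between the cable's end particles and registers a projected energy-cost label with Level3HUD.
; A valid click or touch marks the line used, moves the HUD-held player position and deducts energy, while an out-of-reach click restarts the game.
; Tick swaps materials to highlight selectable and used lines.
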(event OnInputTouchBegin(InputHandler)
  (params (FingerIndex :type ETouchIndex%20Enum :default "Touch1") (TouchedComponent :type Primitive%20Component%20Object%20Reference))
  (bind _currenthud (Variables|Default|GetCurrentHUD))
  (bind _currenthud_2 (Variables|Default|GetCurrentHUD))
  (bind _currenthud_3 (Variables|Default|GetCurrentHUD))
  (bind _difficultylevel (Variables|/Game/Blueprints/Level3/Level3HUD.Level3HUD_C|GetDifficultyLevel _currenthud_2))
  ;[1 1 1] When line handler is clicked/touched set it as used and move current position and deduct energy
  (if (Rendering|IsVisible (Variables|Default|GetCableComponent))
    (if (Variables|Default|GetIsReady)
      (if (Variables|/Game/Blueprints/Level3/Level3HUD.Level3HUD_C|GetHasStartedMovement _currenthud_3)
        (if (< (Math|Vector|Distance(Vector) (Transformation|GetActorLocation (Class|CableComponent|GetAttachedActor (Variables|Default|GetCableComponent))) (Variables|/Game/Blueprints/Level3/Level3HUD.Level3HUD_C|GetCurrentPlayerPosition _currenthud_3)) (Variables|Default|GetCoreCenterOutSafeDistance))
          (Variables|Default|SetHasBeenUsed true :!label _label)
          (Variables|/Game/Blueprints/Level3/Level3HUD.Level3HUD_C|SetCurrentPlayerPosition _currenthud (Transformation|GetWorldLocation (Variables|Default|GetCableComponent)))
          (Variables|/Game/Blueprints/Level3/Level3HUD.Level3HUD_C|SetHasStartedMovement _currenthud true)
          (if (> _difficultylevel 1)
            (if (Variables|Default|GetNeedsDifficultyEnergy)
              (Variables|/Game/Blueprints/Level3/Level3HUD.Level3HUD_C|SetCurrentEnergy (Variables|Default|GetCurrentHUD) (- (Variables|/Game/Blueprints/Level3/Level3HUD.Level3HUD_C|GetCurrentEnergy _currenthud_2) (Math|Conversions|ToFloat(Integer) (Utilities|Array|Get(acopy) (Variables|Default|GetDifficultyEnergyConsumption) _difficultylevel))))
              (else
                (Variables|/Game/Blueprints/Level3/Level3HUD.Level3HUD_C|SetCurrentEnergy _currenthud (- (Variables|/Game/Blueprints/Level3/Level3HUD.Level3HUD_C|GetCurrentEnergy _currenthud) (Math|Conversions|ToFloat(Integer) (Variables|Default|GetEnergyConsumption))) :!label _label_2)))
            (else
              (goto _label_2)))
          (else
            (Default|CallRestartGame _currenthud)
            (Default|ResetGameStatus _currenthud)))
        (elif (Variables|Default|GetIsStartLine)
          (goto _label))))))

(event OnClicked(InputHandler)
  (params (TouchedComponent :type Primitive%20Component%20Object%20Reference) (ButtonPressed :type Key%20Structure :default "None"))
  (bind _currenthud (Variables|Default|GetCurrentHUD))
  (bind _currenthud_2 (Variables|Default|GetCurrentHUD))
  (bind _currenthud_3 (Variables|Default|GetCurrentHUD))
  (bind _difficultylevel (Variables|/Game/Blueprints/Level3/Level3HUD.Level3HUD_C|GetDifficultyLevel _currenthud_2))
  ;[1 1 1] When line handler is clicked/touched set it as used and move current position and deduct energy
  (if (Rendering|IsVisible (Variables|Default|GetCableComponent))
    (if (Variables|Default|GetIsReady)
      (if (Variables|/Game/Blueprints/Level3/Level3HUD.Level3HUD_C|GetHasStartedMovement _currenthud_3)
        (if (< (Math|Vector|Distance(Vector) (Transformation|GetActorLocation (Class|CableComponent|GetAttachedActor (Variables|Default|GetCableComponent))) (Variables|/Game/Blueprints/Level3/Level3HUD.Level3HUD_C|GetCurrentPlayerPosition _currenthud_3)) (Variables|Default|GetCoreCenterOutSafeDistance))
          (Variables|Default|SetHasBeenUsed true :!label _label)
          (Variables|/Game/Blueprints/Level3/Level3HUD.Level3HUD_C|SetCurrentPlayerPosition _currenthud (Transformation|GetWorldLocation (Variables|Default|GetCableComponent)))
          (Variables|/Game/Blueprints/Level3/Level3HUD.Level3HUD_C|SetHasStartedMovement _currenthud true)
          (if (> _difficultylevel 1)
            (if (Variables|Default|GetNeedsDifficultyEnergy)
              (Variables|/Game/Blueprints/Level3/Level3HUD.Level3HUD_C|SetCurrentEnergy (Variables|Default|GetCurrentHUD) (- (Variables|/Game/Blueprints/Level3/Level3HUD.Level3HUD_C|GetCurrentEnergy _currenthud_2) (Math|Conversions|ToFloat(Integer) (Utilities|Array|Get(acopy) (Variables|Default|GetDifficultyEnergyConsumption) _difficultylevel))))
              (else
                (Variables|/Game/Blueprints/Level3/Level3HUD.Level3HUD_C|SetCurrentEnergy _currenthud (- (Variables|/Game/Blueprints/Level3/Level3HUD.Level3HUD_C|GetCurrentEnergy _currenthud) (Math|Conversions|ToFloat(Integer) (Variables|Default|GetEnergyConsumption))) :!label _label_2)))
            (else
              (goto _label_2)))
          (else
            (Default|CallRestartGame _currenthud)
            (Default|ResetGameStatus _currenthud)))
        (elif (Variables|Default|GetIsStartLine)
          (goto _label))))))

(event Custom|OnRestart
  ;[1 1 1] Insert location and value into HUD to be drawn
  (CallFunction|RestartGame))

(event Custom|OnGameFinished
  ;[1 1 1] Insert location and value into HUD to be drawn
  (CallFunction|SetGameOver))

(event EventBeginPlay
  (bind _inputhandlerscale (Variables|Default|GetInputHandlerScale))
  (Utilities|FlowControl|Delay 1.0)
  (Variables|Default|SetHasBeenUsed false)
  (Variables|Default|SetLastHasBeenUsed false)
  (bind _hud (CallFunction|GetUMGHud))
  ;[1 1 1] Get start and end position of cable particles to calculate corresponding cube/inputhandler transform
  (Variables|Default|SetCurrentHUD _hud)
  (bind _output_get (Variables|Default|SetCableParticles (Class|CableComponent|GetCableParticleLocations (Variables|Default|GetCableComponent))))
  (Variables|Default|SetCableStart (Utilities|Array|Get(acopy) _output_get))
  (Variables|Default|SetCableEnd (Utilities|Array|Get(acopy) _output_get (Utilities|Array|LastIndex _output_get)))
  ;[1 1 1] Calculate size, position and rotation for our inputhandler cube to receive click/touch events for reflect cable position
  (bind _angleyaw (CallFunction|CalculateVectorYaw (Variables|Default|GetCableStart) (Variables|Default|GetCableEnd) 9e+01))
  (Transformation|SetWorldRotation (Variables|Default|GetInputHandler) (Math|Rotator|MakeRotator 9e+01 0.0 _angleyaw) false false)
  (Transformation|SetWorldLocation (Variables|Default|GetInputHandler) (/ (+ (Variables|Default|GetCableStart) (Variables|Default|GetCableEnd)) "2.000000,2.000000,2.000000") false false)
  (Transformation|SetWorldScale3D (Variables|Default|GetInputHandler) (Math|Vector|MakeVector _inputhandlerscale _inputhandlerscale (/ (Math|Vector|Distance(Vector) (Variables|Default|GetCableStart) (Variables|Default|GetCableEnd)) 1e+02)))
  ;[1 1 1] Insert location and value into HUD to be drawn
  (if (<= (Variables|Default|GetDifficultyLevel) (Variables|/Game/Blueprints/Level3/Level3HUD.Level3HUD_C|GetDifficultyLevel (Variables|Default|GetCurrentHUD)))
    (if (> (Variables|/Game/Blueprints/Level3/Level3HUD.Level3HUD_C|GetDifficultyLevel (Variables|Default|GetCurrentHUD)) 1)
      (if (Variables|Default|GetNeedsDifficultyEnergy)
        (Utilities|Array|Add (Variables|/Game/Blueprints/Level3/Level3HUD.Level3HUD_C|GetEnergyTextValues (Variables|Default|GetCurrentHUD)) (Utilities|Array|Get(acopy) (Variables|Default|GetDifficultyEnergyConsumption) (Variables|/Game/Blueprints/Level3/Level3HUD.Level3HUD_C|GetDifficultyLevel (Variables|Default|GetCurrentHUD))))
        (else
          (Utilities|Array|Add (Variables|/Game/Blueprints/Level3/Level3HUD.Level3HUD_C|GetEnergyTextValues (Variables|Default|GetCurrentHUD)) (Variables|Default|GetEnergyConsumption) :!label _label)))
      (else
        (goto _label)))
    (Utilities|Array|Add (Variables|/Game/Blueprints/Level3/Level3HUD.Level3HUD_C|GetEnergyTextValuePositions (Variables|Default|GetCurrentHUD)) (Math|Vector2D|MakeVector2D (+ (.X (Math|Vector2D|BreakVector2D (.ScreenPosition (Class|WidgetLayoutLibrary|ProjectWorldLocationtoWidgetPosition (Game|GetPlayerController 0) (/ (+ (Variables|Default|GetCableStart) (Variables|Default|GetCableEnd)) "2.000000,2.000000,2.000000"))))) 2e+01) (.Y (Math|Vector2D|BreakVector2D (.ScreenPosition (Class|WidgetLayoutLibrary|ProjectWorldLocationtoWidgetPosition (Game|GetPlayerController 0) (/ (+ (Variables|Default|GetCableStart) (Variables|Default|GetCableEnd)) "2.000000,2.000000,2.000000")))))))
    (EventDispatchers|BindEventtoRestartGame (Variables|Default|GetCurrentHUD) (delegate Custom|OnRestart))
    (EventDispatchers|BindEventtoGameFinished (Variables|Default|GetCurrentHUD) (delegate Custom|OnGameFinished))
    (Variables|Default|SetIsReady true)
    (if (<= (Variables|Default|GetDifficultyLevel) (Variables|/Game/Blueprints/Level3/Level3HUD.Level3HUD_C|GetDifficultyLevel (Variables|Default|GetCurrentHUD)))
      (Rendering|SetVisibility (Variables|Default|GetCableComponent) true false)
      (else
        (Rendering|SetVisibility (Variables|Default|GetCableComponent) false false)))
    (else
      (Rendering|SetVisibility (Variables|Default|GetCableComponent) false false))))

(event EventTick
  (params (DeltaSeconds :type Float%20%28single-precision%29))
  (bind _hasbeenused (Variables|Default|GetHasBeenUsed))
  (bind _cablecomponent (Variables|Default|GetCableComponent))
  (bind _cablecomponent_2 (Variables|Default|GetCableComponent))
  (bind _currenthud (Variables|Default|GetCurrentHUD))
  (bind _cablecomponent_3 (Variables|Default|GetCableComponent))
  (bind _returnvalue (Class|CableComponent|GetAttachedActor _cablecomponent_3))
  (bind _currentplayerposition (Variables|/Game/Blueprints/Level3/Level3HUD.Level3HUD_C|GetCurrentPlayerPosition _currenthud))
  (if (Variables|Default|GetIsReady)
    ;[1 1 1] Highlight next clickable connections
    (if (Math|Vector|NotEqual(Vector) (Variables|Default|GetLastWorldPosition) _currentplayerposition 0.0001)
      (if true
        (bind _ascore (Utilities|Casting|CastToCore _returnvalue)
          (:then
            (Variables|Default|SetLastWorldPosition _currentplayerposition)
            (if (< (Math|Vector|Distance(Vector) _currentplayerposition (Transformation|GetActorLocation _ascore)) (Variables|Default|GetCoreCenterOutSafeDistance))
              (Rendering|Material|SetMaterial _cablecomponent 0 "/Game/Assets/level3/SelectableLineMaterial.SelectableLineMaterial" :!label _label)
              (else
                (Rendering|Material|SetMaterial _cablecomponent 0 "/Game/Assets/level3/LineMaterial.LineMaterial" :!label _label_2)
                (if (Variables|Default|GetHasBeenUsed)
                  (Rendering|Material|SetMaterial (Variables|Default|GetCableComponent) 0 "/Game/Assets/level3/UsedLineMaterial.UsedLineMaterial")))))
          (:CastFailed
            (Utilities|Casting|CastToLevel3Board _returnvalue)
            (if (Variables|/Game/Blueprints/Level3/Level3HUD.Level3HUD_C|GetHasStartedMovement _currenthud)
              (if (Variables|Default|GetShouldResetStartMaterial)
                (Variables|Default|SetShouldResetStartMaterial false)
                (goto _label_2))
              (elif (not (Variables|Default|GetShouldResetStartMaterial))
                (Variables|Default|SetShouldResetStartMaterial true)
                (goto _label))))))
      (else
        ;[1 1 1] Change line color depending if its been used
        (if (Math|Boolean|NotEqual(Boolean) _hasbeenused (Variables|Default|GetLastHasBeenUsed))
          (if _hasbeenused
            (Rendering|Material|SetMaterial _cablecomponent_2 0 "/Game/Assets/level3/UsedLineMaterial.UsedLineMaterial")
            (else
              (Rendering|Material|SetMaterial _cablecomponent_2 0 "/Game/Assets/level3/LineMaterial.LineMaterial")))
          (Variables|Default|SetLastHasBeenUsed (Variables|Default|GetHasBeenUsed)))))))

(fn ConstructionScript)

(fn CalculateVectorYaw
  (params (Point%20A :type Vector) (Point%20B :type Vector) (Yaw :type Float%20%28single-precision%29))
  (bind (_x _y _z) (Math|Vector|BreakVector Point%20B))
  (bind _returnvalue (Math|Rotator|MakeRotator 1.0 1.0 Yaw))
  (bind _returnvalue_2 (Math|Vector|GetForwardVector _returnvalue))
  (bind _returnvalue_3 (+ _z -1.0))
  (bind _returnvalue_4 (Math|Vector|MakeVector _x _y _returnvalue_3))
  (bind _returnvalue_5 (Math|Vector|Normalize _returnvalue_2))
  (bind _returnvalue_6 (- Point%20A _returnvalue_4))
  (bind _returnvalue_7 (Math|Vector|Normalize _returnvalue_6))
  (if (Variables|Default|GetForceYawDir)
    (Variables|Default|SetYawDir -1.0))
  (return (* (* (Class|KismetMathLibrary|DegAcos (Math|Vector|DotProduct _returnvalue_5 _returnvalue_7)) (Math|Float|Sign(Float) (.Z (Math|Vector|BreakVector (* _returnvalue_5 _returnvalue_7))))) (Variables|Default|GetYawDir))))

(fn RestartGame
  (bind _currenthud (Variables|Default|GetCurrentHUD))
  ;[1 1 1] Set all variables to their starting state
  (Variables|Default|SetHasBeenUsed false)
  (Variables|Default|SetLastHasBeenUsed false)
  (Variables|Default|SetShouldResetStartMaterial false)
  (Variables|Default|SetLastWorldPosition "0, 0, 0")
  (Variables|/Game/Blueprints/Level3/Level3HUD.Level3HUD_C|SetCurrentEnergy _currenthud 15.0)
  (Variables|/Game/Blueprints/Level3/Level3HUD.Level3HUD_C|SetHasStartedMovement _currenthud false)
  (Variables|/Game/Blueprints/Level3/Level3HUD.Level3HUD_C|SetCurrentPlayerPosition _currenthud "-360.000000,-80.000000,-30.000000")
  (Rendering|Material|SetMaterial (Variables|Default|GetCableComponent) 0 "/Game/Assets/level3/LineMaterial.LineMaterial"))

(fn GetUMGHud
  (bind _asgame_3pawn_bp (Utilities|Casting|CastToGame3Pawn_BP (Game|Player|GetPlayerPawn 0)))
  (bind _aslevel_3hud (Utilities|Casting|CastToLevel3HUD (Variables|/Game/Blueprints/Networking/MinigamePawn.MinigamePawn_C|GetHUD _asgame_3pawn_bp)))
  (return _aslevel_3hud))

(fn SetGameOver
  (Variables|Default|SetIsReady false))