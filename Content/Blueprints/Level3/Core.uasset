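; Level 3 Core actor whose Cube mesh is shown or hidden according to the game's difficulty level.
; On BeginPlay it shows the Cube if its own DifficultyLevel is at or below the HUD's DifficultyLevel, otherwise hides it.
; GetUMGHud fetches the Level3HUD by casting the player pawn to Game3Pawn_BP and reading its HUD.
; Only visibility changes; collision is untouched.
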(event EventBeginPlay
  (bind _hud (CallFunction|GetUMGHud))
  ;[1 1 1] Set core visibility hidden if it should not be visible with this difficulty level
  (if (<= (Variables|Default|GetDifficultyLevel) (Variables|/Game/Blueprints/Level3/Level3HUD.Level3HUD_C|GetDifficultyLevel _hud))
    (Rendering|SetVisibility (Variables|Default|GetCube) true false)
    (else
      (Rendering|SetVisibility (Variables|Default|GetCube) false false))))

(event Collision|EventActorBeginOverlap
  (params (OtherActor :type Actor%20Object%20Reference)))

(event EventTick
  (params (DeltaSeconds :type Float%20%28single-precision%29)))

(fn ConstructionScript)

(fn GetUMGHud
  (bind _asgame_3pawn_bp (Utilities|Casting|CastToGame3Pawn_BP (Game|Player|GetPlayerPawn 0)))
  (bind _aslevel_3hud (Utilities|Casting|CastToLevel3HUD (Variables|/Game/Blueprints/Networking/MinigamePawn.MinigamePawn_C|GetHUD _asgame_3pawn_bp)))
  (return _aslevel_3hud))