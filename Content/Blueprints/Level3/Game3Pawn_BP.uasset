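; Player pawn for the Level 3 minigame that sets up each client's HUD and top-down view of the board.
; On BeginPlay it selects the Level 3 HUD class; a non-authority local pawn with a minigame player state then initializes it.
; That pawn also spawns the board locally far below itself, pitches the camera straight down and lowers itself.
; A test input connects to a localhost server, and CheckReadyStatus is an empty stub.
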(event CheckReadyStatus(NetworkController))

(event EventBeginPlay
  (Variables|Default|SetHUDClass "/Game/Blueprints/Level3/Level3HUD.Level3HUD_C")
  (if (== self (Game|Player|GetPlayerPawn 0))
    (Utilities|Casting|CastToMinigame_Playerstate (Variables|Default|GetPlayerState))
    (Networking|SwitchHasAuthority
      (:Remote
        (CallFunction|InitializeHUD)
        (Game|SpawnActorfromClass "/Game/Blueprints/Level3/Level3Board.Level3Board_C" (Math|Transform|MakeTransform (+ (Transformation|GetActorLocation) (Math|Vector|MakeVector 0.0 0.0 -4e+03)) (Math|Rotator|MakeRotator 0.0 0.0 0.0)) "Undefined" 0 0)
        (Pawn|SetControlRotation (Pawn|GetController self) (Math|Rotator|MakeRotator 0.0 -9e+01 0.0))
        (Transformation|AddActorWorldOffset "0, 0,-500.000000")))))

(event Collision|EventActorBeginOverlap
  (params (OtherActor :type Actor%20Object%20Reference)))

(event EventTick
  (params (DeltaSeconds :type Float%20%28single-precision%29)))

(event Input|ActionEvents|InputActionConnectionTest_Server
  (params (Key :type Key%20Structure :default "None")))

(event Input|ActionEvents|InputActionConnectionTest_Client
  (params (Key :type Key%20Structure :default "None"))
  (:Pressed
    (Development|ExecuteConsoleCommand "open 127.0.0.1" (Game|GetPlayerController 0))))

(fn ConstructionScript)