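; Game board actor for the Level 3 minigame that builds a puzzle of cores and cable lines at startup.
; It reads difficulty from the player state, caps it at 2 on the HUD, then resizes and shifts the board.
; Cores and lines spawn cumulatively per difficulty from flattened-height arrays, with cables attached to cores or board attachment points.
; It also sets the HUD's goal X and signals game start to the server.
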(event EventBeginPlay
  (bind _generator (Variables|Default|GetGenerator))
  (CallFunction|PopulateAttachmentPoints)
  (Utilities|FlowControl|Delay 0.2)
  ;[1 1 1] Set board scaling and position based on difficulty level
  (bind _hud (CallFunction|GetUMGHud))
  (bind _difficulty (CallFunction|GetDifficultyLevel))
  (Variables|Default|SetCurrentDifficulty _difficulty)
  (CallFunction|ForceHeight)
  (if (== (Variables|/Game/Blueprints/Level3/Level3HUD.Level3HUD_C|GetDifficultyLevel _hud) 0)
    (Transformation|SetWorldScale3D (Variables|Default|GetGround) (Math|Vector|MakeVector (.X (Math|Vector2D|BreakVector2D (Variables|Default|GetSize))) (.Y (Math|Vector2D|BreakVector2D (Variables|Default|GetSize))) 1.0) :!label _label)
    (Transformation|SetWorldScale3D _generator (Math|Vector|MakeVector 3.0 (.Y (Math|Vector2D|BreakVector2D (Variables|Default|GetSize))) 4.0))
    (Transformation|SetWorldScale3D (Variables|Default|GetRepulsionEngine) (Math|Vector|MakeVector 3.0 (.Y (Math|Vector2D|BreakVector2D (Variables|Default|GetSize))) 4.0))
    (Rendering|SetVisibility _generator true false)
    ;[1 1 1] Spawn cores and connectine lines based on difficulty and indicate game start to server
    (CallFunction|SpawnCoresfromArray (Variables|Default|GetCorePositions))
    (if (> (Variables|Default|GetCurrentDifficulty) 0)
      (Variables|Default|SetLineOffset "0,-250.000000, 0")
      (CallFunction|SpawnCoresfromArray (Variables|Default|GetCorePositionsDifficulty_1))
      (if (> (Variables|Default|GetCurrentDifficulty) 1)
        (Variables|Default|SetLineOffset "350.000000,-250.000000, 0")
        (CallFunction|SpawnCoresfromArray (Variables|Default|GetCorePositionsDiffuculty_2))
        (CallFunction|SpawnConnectiveLines)
        (CallFunction|SetServerStart)
        (else
          (CallFunction|SpawnConnectiveLines)
          (CallFunction|SetServerStart)))
      (else
        (CallFunction|SpawnConnectiveLines)
        (CallFunction|SetServerStart)))
    (elif (== (Variables|/Game/Blueprints/Level3/Level3HUD.Level3HUD_C|GetDifficultyLevel _hud) 1)
      (Variables|Default|SetSize "(X=25.000000,Y=40.000000)")
      (Transformation|AddWorldOffset (Variables|Default|GetGround) "0.000000,-250.000000, 0" false true)
      (goto _label)
      (elif (== (Variables|/Game/Blueprints/Level3/Level3HUD.Level3HUD_C|GetDifficultyLevel _hud) 2)
        (Variables|Default|SetSize "(X=32.000000,Y=40.000000)")
        (Transformation|AddWorldOffset (Variables|Default|GetGround) "350.000000,-250.000000, 0" false true)
        (goto _label)))))

(event Collision|EventActorBeginOverlap
  (params (OtherActor :type Actor%20Object%20Reference)))

(event EventTick
  (params (DeltaSeconds :type Float%20%28single-precision%29)))

(fn ConstructionScript)

(fn GetUMGHud
  (bind _returnvalue (Game|GetPlayerController 0))
  ;[1 1 1] Get Hud reference from server set pawn
  (bind _asgame_3pawn_bp (Utilities|Casting|CastToGame3Pawn_BP (Game|Player|GetPlayerPawn 0)))
  (bind _aslevel_3hud (Utilities|Casting|CastToLevel3HUD (Variables|/Game/Blueprints/Networking/MinigamePawn.MinigamePawn_C|GetHUD _asgame_3pawn_bp)))
  (Variables|/Script/Engine.PlayerController|SetbEnableClickEvents _returnvalue true)
  (Variables|/Script/Engine.PlayerController|SetbEnableTouchEvents _returnvalue true)
  (return _aslevel_3hud))

(fn SpawnCoresfromArray
  (params (in_vectors :type Array%20of%20Vectors))
  (bind _currentdifficulty (Variables|Default|GetCurrentDifficulty))
  (bind _arrayelement (Utilities|Array|ReverseforEachLoop in_vectors)
    (:LoopBody
      (if (== _currentdifficulty 1)
        ;[1 1 1] Spawn difficulty  level 1 cores with scaled positions
        (bind _returnvalue (Game|SpawnActorfromClass "/Game/Blueprints/Level3/Core.Core_C" (Math|Transform|MakeTransform (- (+ (Transformation|GetWorldLocation (Variables|Default|GetGround)) _arrayelement) "0,-250.000000, 0")) "Undefined" 0 0))
        (Utilities|Array|Add (Variables|Default|GetCoreCollection) _returnvalue)
        (elif (== _currentdifficulty 2)
          ;[1 1 1] Spawn difficulty level 2 cores with scaled positions
          (bind _returnvalue_2 (Game|SpawnActorfromClass "/Game/Blueprints/Level3/Core.Core_C" (Math|Transform|MakeTransform (- (+ (Transformation|GetWorldLocation (Variables|Default|GetGround)) _arrayelement) "350.000000,-250.000000, 0")) "Undefined" 0 0))
          (Utilities|Array|Add (Variables|Default|GetCoreCollection) _returnvalue_2)
          (else
            ;[1 1 1] Spawn difficulty level 0 cores witout new scaling
            (bind _returnvalue_3 (Game|SpawnActorfromClass "/Game/Blueprints/Level3/Core.Core_C" (Math|Transform|MakeTransform (+ (Transformation|GetWorldLocation (Variables|Default|GetGround)) _arrayelement)) "Undefined" 0 0))
            (Utilities|Array|Add (Variables|Default|GetCoreCollection) _returnvalue_3)))))))

(fn GetDifficultyLevel
  ;[1 1 1] Get difficulty level from server and set it in HUD variable which will be referenced in other blueprints and clamp difficulty level to max 2
  (bind _asminigame_playerstate (Utilities|Casting|CastToMinigame_Playerstate (Variables|/Script/Engine.Controller|GetPlayerState (Game|GetPlayerController 0))))
  (if (> (Variables|/Game/Blueprints/Server/Minigame_Playerstate.Minigame_Playerstate_C|GetDifficultyLevel _asminigame_playerstate) 2)
    (bind _hud (CallFunction|GetUMGHud))
    (Variables|/Game/Blueprints/Level3/Level3HUD.Level3HUD_C|SetDifficultyLevel _hud 2)
    (else
      (bind _hud_2 (CallFunction|GetUMGHud))
      (Variables|/Game/Blueprints/Level3/Level3HUD.Level3HUD_C|SetDifficultyLevel _hud_2 (Variables|/Game/Blueprints/Server/Minigame_Playerstate.Minigame_Playerstate_C|GetDifficultyLevel _asminigame_playerstate))))
  (bind _hud_3 (CallFunction|GetUMGHud))
  (return (Variables|/Game/Blueprints/Level3/Level3HUD.Level3HUD_C|GetDifficultyLevel _hud_3)))

(fn SpawnConnectiveLines
  (CallFunction|ScaleAttachmentPoints)
  (for _array_element (Variables|Default|GetLineData)
    ;[1 1 1] Spawn all connective lines from structure and set all it's variables
    (bind _returnvalue (Game|SpawnActorfromClass "/Game/Blueprints/Level3/ConnectiveLine.ConnectiveLine_C" (Math|Transform|MakeTransform (- (+ (.Position (Utilities|Struct|BreakLineDataStruct _array_element)) (Transformation|GetWorldLocation (Variables|Default|GetGround))) (Variables|Default|GetLineOffset))) "Undefined" 0 0))
    (Utilities|Array|Add (Variables|Default|GetLineCollection) _returnvalue)
    (Variables|/Game/Blueprints/Level3/ConnectiveLine.ConnectiveLine_C|SetEnergyConsumption _returnvalue (.EnergyConsumption (Utilities|Struct|BreakLineDataStruct _array_element)))
    (bind _output_get (Variables|/Game/Blueprints/Level3/ConnectiveLine.ConnectiveLine_C|SetIsStartLine _returnvalue (.IsStartLine (Utilities|Struct|BreakLineDataStruct _array_element))))
    (Variables|/Game/Blueprints/Level3/ConnectiveLine.ConnectiveLine_C|SetDifficultyLevel _returnvalue (.DifficultyLevel (Utilities|Struct|BreakLineDataStruct _array_element)))
    (Variables|/Game/Blueprints/Level3/ConnectiveLine.ConnectiveLine_C|SetDifficultyEnergyConsumption _returnvalue (.DifficultyEnergyConsumption (Utilities|Struct|BreakLineDataStruct _array_element)))
    (Variables|/Game/Blueprints/Level3/ConnectiveLine.ConnectiveLine_C|SetNeedsDifficultyEnergy _returnvalue (.NeedsDifficultyEnergy (Utilities|Struct|BreakLineDataStruct _array_element)))
    (Variables|/Game/Blueprints/Level3/ConnectiveLine.ConnectiveLine_C|SetForceYawDir _returnvalue (.ForceYaw (Utilities|Struct|BreakLineDataStruct _array_element)))
    (if _output_get
      (Class|CableComponent|SetAttachEndtoComponent (Variables|/Script/CableComponent.CableActor|GetCableComponent _returnvalue) (Utilities|Array|Get(acopy) (Variables|Default|GetAttachmentPoints) (Variables|Default|GetAttachmentPointIndex)) "None")
      (Variables|Default|SetAttachmentPointIndex (+ (Variables|Default|GetAttachmentPointIndex) 1))
      (else
        (Class|CableComponent|SetAttachEndto (Variables|/Script/CableComponent.CableActor|GetCableComponent _returnvalue) (Utilities|Array|Get(acopy) (Variables|Default|GetCoreCollection) (.AttachmentIndex (Utilities|Struct|BreakLineDataStruct _array_element))) "None" "None")))))

(fn PopulateAttachmentPoints
  (bind _attachmentpoints (Variables|Default|GetAttachmentPoints))
  ;[1 1 1] Add all attachment points to array to be referenced later on
  (Utilities|Array|Add _attachmentpoints (Variables|Default|GetAttachmentPoint_1))
  (Utilities|Array|Add _attachmentpoints (Variables|Default|GetAttachmentPoint_2))
  (Utilities|Array|Add _attachmentpoints (Variables|Default|GetAttachmentPoint_3))
  (Utilities|Array|Add _attachmentpoints (Variables|Default|GetAttachmentPoint_4)))

(fn ForceHeight
  (bind _corepositions (Variables|Default|GetCorePositions))
  (bind _corepositionsdifficulty_1 (Variables|Default|GetCorePositionsDifficulty_1))
  (bind _corepositionsdiffuculty_2 (Variables|Default|GetCorePositionsDiffuculty_2))
  (bind _linedata (Variables|Default|GetLineData))
  (bind _currentdifficulty (Variables|Default|GetCurrentDifficulty))
  ;[1 1 1] Loop all 3 difficulty level core arrays and set the z (height) on all positions to be the same
  (for (_array_element _array_index) _corepositions
    (Utilities|Array|SetArrayElem _corepositions _array_index (Math|Vector|MakeVector (.X (Math|Vector|BreakVector _array_element)) (.Y (Math|Vector|BreakVector _array_element)) (Variables|Default|GetGoalHeight))))
  (for (_array_element_2 _array_index_2) _corepositionsdifficulty_1
    (Utilities|Array|SetArrayElem _corepositionsdifficulty_1 _array_index_2 (Math|Vector|MakeVector (.X (Math|Vector|BreakVector _array_element_2)) (.Y (Math|Vector|BreakVector _array_element_2)) (Variables|Default|GetGoalHeight))))
  (for (_array_element_3 _array_index_3) _corepositionsdiffuculty_2
    (Utilities|Array|SetArrayElem _corepositionsdiffuculty_2 _array_index_3 (Math|Vector|MakeVector (.X (Math|Vector|BreakVector _array_element_3)) (.Y (Math|Vector|BreakVector _array_element_3)) (Variables|Default|GetGoalHeight))))
  ;[1 1 1] Merge needed connective line arrays based on difficulty
  (if (== _currentdifficulty 1)
    (Utilities|Array|AppendArray (Variables|Default|GetLineData) (Variables|Default|GetLineDataDifficulty_1))
    (elif (== _currentdifficulty 2)
      (Utilities|Array|AppendArray (Variables|Default|GetLineData) (Variables|Default|GetLineDataDifficulty_1))
      (Utilities|Array|AppendArray (Variables|Default|GetLineData) (Variables|Default|GetLineDataDifficulty_2))))
  ;[1 1 1] Loop all connective lines and set their z (height) to be same as core height's
  (for (_array_element_4 _array_index_4) _linedata
    (Utilities|Array|SetArrayElem _linedata _array_index_4 (Utilities|Struct|MakeLineDataStruct (Math|Vector|MakeVector (.X (Math|Vector|BreakVector (.Position (Utilities|Struct|BreakLineDataStruct _array_element_4)))) (.Y (Math|Vector|BreakVector (.Position (Utilities|Struct|BreakLineDataStruct _array_element_4)))) (Variables|Default|GetGoalHeight)) (.EnergyConsumption (Utilities|Struct|BreakLineDataStruct _array_element_4)) (.IsStartLine (Utilities|Struct|BreakLineDataStruct _array_element_4)) (.DifficultyLevel (Utilities|Struct|BreakLineDataStruct _array_element_4)) (.DifficultyEnergyConsumption (Utilities|Struct|BreakLineDataStruct _array_element_4)) (.NeedsDifficultyEnergy (Utilities|Struct|BreakLineDataStruct _array_element_4)) (.AttachmentIndex (Utilities|Struct|BreakLineDataStruct _array_element_4)) (.AttachmentOffset (Utilities|Struct|BreakLineDataStruct _array_element_4)) (.ForceYaw (Utilities|Struct|BreakLineDataStruct _array_element_4)))))
  ;[1 1 1] Set the goal x axis which will indicate player has reached the other side of the baord
  (bind _hud (CallFunction|GetUMGHud))
  (if (> (Variables|Default|GetCurrentDifficulty) 1)
    (Variables|Default|SetTargetXAxis 1.73e+03))
  (Variables|/Game/Blueprints/Level3/Level3HUD.Level3HUD_C|SetGoalXAxis _hud (+ (.X (Math|Vector|BreakVector (Transformation|GetWorldLocation (Variables|Default|GetGround)))) (Variables|Default|GetTargetXAxis))))

(fn ScaleAttachmentPoints
  (if (> (Variables|Default|GetCurrentDifficulty) 0)
    ;[1 1 1] Scale attachmentpoint positions if difficulty is greater then 0 to match the map scaling
    (Transformation|AddWorldOffset (Variables|Default|GetAttachmentPoint_2) (Math|Vector|MakeVector 0.0 2e+02 0.0) false true)
    (Transformation|AddWorldOffset (Variables|Default|GetAttachmentPoint_3) (Math|Vector|MakeVector 0.0 7e+02 0.0) false true)
    (Transformation|AddWorldOffset (Variables|Default|GetAttachmentPoint_1) "0,-150.000000, 0" false true)
    (Transformation|AddWorldOffset (Variables|Default|GetAttachmentPoint_4) "0,350.000000, 0" false true)
    (else
      ;[1 1 1] Scale attachmentpoint positions if difficulty is 0
      (Transformation|AddWorldOffset (Variables|Default|GetAttachmentPoint_2) (Math|Vector|MakeVector 0.0 0.0 0.0) false true)
      (Transformation|AddWorldOffset (Variables|Default|GetAttachmentPoint_3) (Math|Vector|MakeVector 0.0 2e+02 0.0) false true)
      (Transformation|AddWorldOffset (Variables|Default|GetAttachmentPoint_1) "0,-150.000000, 0" false true))))

(fn SetServerStart
  ;[1 1 1] Send progression status to server to indicate that we have started the game
  (bind _asminigame_state (Utilities|Casting|CastToMinigameState (Variables|/Script/Engine.Controller|GetPlayerState (Game|GetPlayerController 0))))
  (Class|MinigameState|ServerRPCTaskComplete _asminigame_state 0.0)
  (return))