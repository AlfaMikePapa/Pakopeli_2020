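; Tile actor with a boolean life state, shown through the colour and brightness of its emissive material.
; ChangeColor flips the state and sets targets: bright green when false, dimmer red when true.
; Tick eases the current values toward those targets and writes them to material parameters until both are nearly equal.
; Clicking the tile separately swaps its material between two assets without changing the state.
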(event OnClicked(Tile)
  (params (TouchedComponent :type Primitive%20Component%20Object%20Reference) (ButtonPressed :type Key%20Structure :default "None"))
  (if (== (Rendering|Material|GetMaterial TouchedComponent 0) "/Game/Geometry/Meshes/CubeMaterial.CubeMaterial")
    (Rendering|Material|SetMaterial TouchedComponent 0 "/Game/FirstPerson/Meshes/FirstPersonProjectileMaterial.FirstPersonProjectileMaterial")
    (else
      (Rendering|Material|SetMaterial TouchedComponent 0 "/Game/Geometry/Meshes/CubeMaterial.CubeMaterial"))))

(event OnInputTouchBegin(Tile)
  (params (FingerIndex :type ETouchIndex%20Enum :default "Touch1") (TouchedComponent :type Primitive%20Component%20Object%20Reference)))

(event Collision|EventActorBeginOverlap
  (params (OtherActor :type Actor%20Object%20Reference)))

(event EventTick
  (params (DeltaSeconds :type Float%20%28single-precision%29))
  ;[1 1 1] Check if anything needs interpolating
  (if (not (and (Class|KismetMathLibrary|LinearColorIsNearEqual (Variables|Default|GetColourCurrent) (Variables|Default|GetColourTarget) 0.01) (Math|Float|NearlyEqual(Float) (Variables|Default|GetBrightnessTarget) (Variables|Default|GetBrightnessCurrent) 0.01)))
    ;[1 1 1] Interpolate Colour
    (Rendering|Material|SetVectorParameterValueonMaterials (Variables|Default|GetTile) "EmissionTint" (Math|Conversions|ToVector(LinearColor) (Class|KismetMathLibrary|CInterpto (Variables|Default|GetColourCurrent) (Variables|Default|GetColourTarget) DeltaSeconds (Variables|Default|GetInterpolationSpeed))))
    (Variables|Default|SetColourCurrent (Class|KismetMathLibrary|CInterpto (Variables|Default|GetColourCurrent) (Variables|Default|GetColourTarget) DeltaSeconds (Variables|Default|GetInterpolationSpeed)))
    ;[1 1 1] InterpolateBrightness
    (Rendering|Material|SetScalarParameterValueonMaterials (Variables|Default|GetTile) "EmissionBrightness" (Math|Interpolation|FInterpTo (Variables|Default|GetBrightnessCurrent) (Variables|Default|GetBrightnessTarget) DeltaSeconds 12.0))
    (Variables|Default|SetBrightnessCurrent (Math|Interpolation|FInterpTo (Variables|Default|GetBrightnessCurrent) (Variables|Default|GetBrightnessTarget) DeltaSeconds 12.0))))

(event EventBeginPlay)

(fn ConstructionScript)

(fn ChangeColor
  (if (Variables|Default|GetLifeState)
    (Variables|Default|SetLifeState false)
    ;[1 1 1] SetColourTargetGreen
    (Variables|Default|SetColourTarget (Utilities|Struct|MakeLinearColor 0.0 1.0 0.0 0.0))
    (Variables|Default|SetInterpolationSpeed 3.0)
    ;[1 1 1] Set Brightness Target, Flash
    (Variables|Default|SetBrightnessTarget 3e+01)
    (else
      (Variables|Default|SetLifeState true)
      ;[1 1 1] SetColourTargetRed
      (Variables|Default|SetColourTarget (Utilities|Struct|MakeLinearColor 1.0 0.0 0.0 0.0))
      (Variables|Default|SetInterpolationSpeed 3.0)
      ;[1 1 1] Set Brightness Target, Flash
      (Variables|Default|SetBrightnessTarget 2.0))))