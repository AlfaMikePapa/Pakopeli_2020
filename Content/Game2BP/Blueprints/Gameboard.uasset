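; Gameboard actor for a tile-toggle puzzle minigame where the player reproduces a goal pattern.
; SpawnEvent builds player and goal tile grids, scrambles the goal with Difficulty random row/column flips, and spawns local light and volumetric fog.
; ExecuteMoves replays queued moves with delays via index maps, then BoardComparison checks tile states against the goal and reports through Game2Pawn_BP.
; ResetFunction clears the player board but is not called here.
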(event Custom|SpawnEvent
  (params (Difficulty :type Integer))
  (bind _maxx (Variables|Default|GetMaxX))
  (bind _maxy (Variables|Default|GetMaxY))
  (bind _maxy_2 (Variables|Default|GetMaxY))
  (bind _tilesize (Variables|Default|GetTileSize))
  (bind _maxy_3 (Variables|Default|GetMaxY))
  (bind _tilesize_2 (Variables|Default|GetTileSize))
  (bind _returnvalue (* _maxx _maxy))
  (bind _returnvalue_2 (- _returnvalue 1))
  ;[1 1 1] Player gameboard spawn
  (Variables|Default|SetSetDifficulty Difficulty)
  (Utilities|Array|Resize (Variables|Default|GetTileArray) _returnvalue)
  (for _index (range 0 _returnvalue_2)
    (bind _returnvalue_3 (Game|SpawnActorfromClass "/Game/Game2BP/Blueprints/Tile.Tile_C" (Math|Conversions|ToTransform(Vector) (Math|Vector|MakeVector (Math|Conversions|ToFloat(Integer) (* (/ _index _maxy_2) _tilesize)) (Math|Conversions|ToFloat(Integer) (* (Math|Integer|%(Integer) _index _maxy_2) _tilesize)) 0.0)) "AlwaysSpawn" 0 _index 0))
    (Default|ChangeColor _returnvalue_3)
    (Transformation|AttachComponentToComponent _returnvalue_3 (Variables|Default|GetPlayerBoardRoot) "None" "KeepRelative" "KeepRelative" "KeepRelative" true)
    (Utilities|Array|SetArrayElem (Variables|Default|GetTileArray) _index _returnvalue_3))
  ;[1 1 1] Goal board spawn  and generation (move to its own function?)
  (Utilities|Array|Resize (Variables|Default|GetGoalArray) _returnvalue)
  (for _index_2 (range 0 _returnvalue_2)
    (bind _returnvalue_4 (Game|SpawnActorfromClass "/Game/Game2BP/Blueprints/Tile.Tile_C" (Math|Conversions|ToTransform(Vector) (+ (Math|Vector|MakeVector (Math|Conversions|ToFloat(Integer) (* (/ _index_2 _maxy_3) _tilesize_2)) (Math|Conversions|ToFloat(Integer) (* (Math|Integer|%(Integer) _index_2 _maxy_3) _tilesize_2)) 0.0) (Transformation|GetWorldLocation (Variables|Default|GetGoalBoardRoot)))) "Undefined" 0 _index_2 0))
    (Default|ChangeColor _returnvalue_4)
    (Rendering|LOD|SetForcedLodModel (Variables|/Game/Game2BP/Blueprints/Tile.Tile_C|GetTile _returnvalue_4) 4)
    (Transformation|AttachComponentToComponent _returnvalue_4 (Variables|Default|GetGoalBoardRoot) "None" "KeepRelative" "KeepRelative" "KeepRelative" true)
    (Utilities|Array|SetArrayElem (Variables|Default|GetGoalArray) _index_2 _returnvalue_4))
  (bind (_movequeue _orientation) (CallFunction|RandomWinState (Variables|Default|GetSetDifficulty)))
  (CallFunction|GenerateGoal _movequeue _orientation)
  ;[1 1 1] Setting up fog and lights
  (CallFunction|GameboardGraphicsSetup))

(event Custom|Execute%20Moves
  (params (Moves :type Array%20of%20Integers))
  (bind _tilearray (Variables|Default|GetTileArray))
  ;[1 1 1] Activates gameboard tiles from command queue coming from Pawn < UI
  (for _array_element Moves
    (if (< _array_element 5)
      (CallFunction|ActivateRowX (+ _array_element 1) _tilearray)
      (Utilities|FlowControl|Delay 0.4)
      (else
        (CallFunction|ActivateRowY (.Value (Utilities|Map|Find (Variables|Default|GetYRowMap) _array_element)) _tilearray)
        (Utilities|FlowControl|Delay 0.4))))
  (CallFunction|BoardComparison))

(event EventBeginPlay)

(event Collision|EventActorBeginOverlap
  (params (OtherActor :type Actor%20Object%20Reference)))

(event EventTick
  (params (DeltaSeconds :type Float%20%28single-precision%29)))

(fn ConstructionScript
  ;[1 1 1] Map to assist activation of indexes
  (Utilities|Map|Add (Variables|Default|GetHRowMap) 1 0)
  (for _index (range 2 (Variables|Default|GetMaxY))
    (bind _output_get (LocalVariables|SetMapIndexHelper (+ (LocalVariables|GetMapIndexHelper) (Variables|Default|GetMaxX))))
    (Utilities|Map|Add (Variables|Default|GetHRowMap) _index _output_get))
  ;[1 1 1] Assist map for Y indexes
  (for _index_2 (range 5 9)
    (bind _result (Math|Integer|IncrementInt (LocalVariables|GetYIndexHelper))
      (:%20%20
        (Utilities|Map|Add (Variables|Default|GetYRowMap) _index_2 _result)))))

(fn ActivateRowY
  (params (Row :type Integer) (TargetTileArray :type Array%20of%20Tile%20Object%20References))
  (if (<= Row (Variables|Default|GetMaxX))
    (Utilities|Array|SetArrayElem (Variables|Default|GetIndexArray) 0 (- Row 1) true)
    (for _index (range 1 (- (Variables|Default|GetMaxY) 1))
      (Utilities|Array|SetArrayElem (Variables|Default|GetIndexArray) _index (+ (- Row 1) (* _index (Variables|Default|GetMaxX))) true))
    (for _array_element (Variables|Default|GetIndexArray)
      (Default|ChangeColor (Utilities|Array|Get(acopy) TargetTileArray _array_element)))
    (else
      (Development|PrintString "Given row out of bounds!!" true true "(R=0.000000,G=0.660000,B=1.000000,A=1.000000)" 5.0))))

(fn ActivateRowX
  (params (Row :type Integer) (TargetTileArray :type Array%20of%20Tile%20Object%20References))
  (bind _hrowmap (Variables|Default|GetHRowMap))
  (bind (_value _returnvalue) (Utilities|Map|Find _hrowmap Row))
  (if (<= Row (Variables|Default|GetMaxX))
    (if _returnvalue
      (for _index (range _value (+ _value (- (Variables|Default|GetMaxX) 1)))
        (Default|ChangeColor (Utilities|Array|Get(acopy) TargetTileArray _index)))
      (else
        (Development|PrintString "Index not found in map")))
    (else
      (Development|PrintString "HRow Index too large!"))))

(fn GenerateGoal
  (params (MoveQueue :type Array%20of%20Integers) (Orientation :type Array%20of%20Names))
  (bind _goalarray (Variables|Default|GetGoalArray))
  (bind _goalarray_2 (Variables|Default|GetGoalArray))
  ;[1 1 1] Activates row X or Y as generated fro Random Win Sate
  (for (_array_element _array_index) MoveQueue
    (if (Utilities|Name|Equal(Name) (Utilities|Array|Get(acopy) Orientation _array_index) "X")
      (CallFunction|ActivateRowX _array_element _goalarray)
      (else
        (CallFunction|ActivateRowY _array_element _goalarray))))
  ;[1 1 1] Collects goal state
  (Utilities|Array|Resize (Variables|Default|GetGoalState) (Utilities|Array|Length _goalarray_2))
  (for (_array_element_2 _array_index_2) _goalarray_2
    (Utilities|Array|SetArrayElem (Variables|Default|GetGoalState) _array_index_2 (Variables|/Game/Game2BP/Blueprints/Tile.Tile_C|GetLifeState _array_element_2))))

(fn RandomWinState
  (params (GoalMoveCount :type Integer))
  (bind _orientation (Variables|Default|GetOrientation))
  (Utilities|Array|Resize (Variables|Default|GetMoveQueue) GoalMoveCount)
  (Utilities|Array|Resize (Variables|Default|GetOrientation) GoalMoveCount)
  (for _index (range 0 (- GoalMoveCount 1))
    ;[1 1 1] Generates move indexes without 2 of the same integers in a row
    (while (== (stale _output_get) (LocalVariables|GetPreviousMoveIndex))
      (bind _output_get (LocalVariables|SetCurrentRandom (Math|Random|RandomIntegerinRange 1 (Variables|Default|GetMaxX)))))
    (bind _output_get_2 (LocalVariables|SetPreviousMoveIndex (LocalVariables|GetCurrentRandom)))
    (Utilities|Array|SetArrayElem (Variables|Default|GetMoveQueue) _index _output_get_2)
    ;[1 1 1] Generates a random X or Y
    (if (Math|Random|RandomBool)
      (Utilities|Array|SetArrayElem _orientation _index "X")
      (else
        (Utilities|Array|SetArrayElem _orientation _index "Y"))))
  (return (Variables|Default|GetMoveQueue) (Variables|Default|GetOrientation)))

(fn BoardComparison
  ;[1 1 1] Collects current Gameboard state (which tiles are activated)
  (Utilities|Array|Resize (Variables|Default|GetBoardState) (* (Variables|Default|GetMaxX) (Variables|Default|GetMaxY)))
  (for (_array_element _array_index) (Variables|Default|GetTileArray)
    (Utilities|Array|SetArrayElem (Variables|Default|GetBoardState) _array_index (Variables|/Game/Game2BP/Blueprints/Tile.Tile_C|GetLifeState _array_element)))
  ;[1 1 1] Compares gameboard to goalboard state
  (for (_array_element_2 _array_index_2) (Variables|Default|GetBoardState)
    (if (not (Math|Boolean|Equal(Boolean) _array_element_2 (Utilities|Array|Get(acopy) (Variables|Default|GetGoalState) _array_index_2)))
      (LocalVariables|SetIsCorrect false)))
  (if (LocalVariables|GetIsCorrect)
    ;[1 1 1] If solution is correct sends completed gamestate for server
    (Development|PrintString "Solution correct!" true true "(R=0.000000,G=0.660000,B=1.000000,A=1.000000)" 2e+01)
    (bind _asgame_2pawn_bp (Utilities|Casting|CastToGame2Pawn_BP (Pawn|GetControlledPawn (Game|GetPlayerController 0)))
      (:then
        (Default|UpdateGameState _asgame_2pawn_bp 1.0))
      (:CastFailed
        (Development|PrintString "Cast to Minigame2Pawn failed" true true "(R=0.000000,G=0.660000,B=1.000000,A=1.000000)" 2e+01)))
    (else
      ;[1 1 1] If solution is incorrect resets gamestate for server and resets the board
      (Development|PrintString "Solution incorrect!" true true "(R=0.000000,G=0.660000,B=1.000000,A=1.000000)" 2e+01)
      (bind _asgame_2pawn_bp_2 (Utilities|Casting|CastToGame2Pawn_BP (Pawn|GetControlledPawn (Game|GetPlayerController 0)))
        (:then
          (Default|UpdateGameState _asgame_2pawn_bp_2 0.5))
        (:CastFailed
          (Development|PrintString "Cast to Minigame2Pawn failed!" true true "(R=0.000000,G=0.660000,B=1.000000,A=1.000000)" 2e+01))))))

(fn GameboardGraphicsSetup
  ;[1 1 1] Local graphics setup
  (bind _returnvalue (Game|SpawnActorfromClass "/Script/Engine.DirectionalLight" (Math|Transform|MakeTransform (Math|Vector|MakeVector 2.8e+02 -2.8e+02 2.4e+02) (Math|Rotator|MakeRotator -1e+01 -17.0 155.0) "2.500000,2.500000,2.500000") "AlwaysSpawn" 0 0))
  (Utilities|FlowControl|Sequence
    (:then_0
      (Rendering|Components|Light|SetCastShadows (Variables|/Script/Engine.Light|GetLightComponent _returnvalue) false)
      (Rendering|Components|Light|SetLightColor (Variables|/Script/Engine.Light|GetLightComponent _returnvalue) "(R=1.000000,G=0.947307,B=0.822786,A=1.000000)" true))
    (:then_1
      (Rendering|Components|Light|SetIntensity (Variables|/Script/Engine.Light|GetLightComponent _returnvalue) 2.0))
    (:then_2
      (bind _returnvalue_2 (Game|SpawnActorfromClass "/Script/Engine.ExponentialHeightFog" (Math|Conversions|ToTransform(Vector) (Math|Vector|MakeVector 164.0 -53.0 5e+01)) "AlwaysSpawn" 0 0))
      (Class|ExponentialHeightFogComponent|SetFogInscatteringColor (Variables|/Script/Engine.ExponentialHeightFog|GetComponent _returnvalue_2) "(R=0.000000,G=0.000000,B=0.000000,A=1.000000)")
      (Class|ExponentialHeightFogComponent|SetVolumetricFog (Variables|/Script/Engine.ExponentialHeightFog|GetComponent _returnvalue_2) true)
      (Class|ExponentialHeightFogComponent|SetVolumetricFogAlbedo (Variables|/Script/Engine.ExponentialHeightFog|GetComponent _returnvalue_2) (Class|KismetMathLibrary|LinearColorQuantize "(R=0.445201,G=0.456411,B=0.686686,A=1.000000)"))
      (Class|ExponentialHeightFogComponent|SetVolumetricFogEmissive (Variables|/Script/Engine.ExponentialHeightFog|GetComponent _returnvalue_2) "(R=0.102242,G=0.097587,B=0.171441,A=0.000000)")
      (Class|ExponentialHeightFogComponent|SetVolumetricFogExtinctionScale (Variables|/Script/Engine.ExponentialHeightFog|GetComponent _returnvalue_2) 3.588572))))

(fn ResetFunction
  (for _array_element (Variables|Default|GetTileArray)
    (if (Variables|/Game/Game2BP/Blueprints/Tile.Tile_C|GetLifeState _array_element)
      (Default|ChangeColor _array_element))))